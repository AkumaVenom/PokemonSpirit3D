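; Electrode pet Blueprint that the player summons through UseItem on MasterCharacter_BP and that self-destructs when it rains.
; BeginPlay caches the level's Weather_BP, and Tick polls its IsRaining flag behind a DoOnce.
; After a random delay it plays a cry, then a large explosion effect and sound, hides its mesh and destroys itself.
; The random gate has weight 1.0, so rain always triggers the explosion.
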(event EventBeginPlay
  (|CallParentFunction)
  (bind _outactors (Actor|GetAllActorsOfClass "/Game/Dynamic_Weather/Blueprints/Weather_BP.Weather_BP_C"))
  (Variables|Default|SetWeatherBP (Utilities|Array|Get(acopy) _outactors)))

(event Collision|EventActorBeginOverlap
  (params (OtherActor :type Actor%20Object%20Reference))
  (|CallParentFunction OtherActor) ; This node is disabled and will not be called.\nDrag off pins to build functionality.
)

(event EventTick
  (params (DeltaSeconds :type Float%20%28single-precision%29))
  (bind _self self)
  (bind _returnvalue (Transformation|GetActorLocation _self))
  (|CallParentFunction DeltaSeconds)
  (bind _weatherbp (Variables|Default|GetWeatherBP)
    (:then
      (if (Variables|/Game/Dynamic_Weather/Blueprints/Weather_BP.Weather_BP_C|GetIsRaining _weatherbp)
        (Utilities|FlowControl|DoOnce false
          (:Completed
            (if (Math|Random|RandomBoolwithWeight 1.0)
              (Utilities|FlowControl|Delay (Math|Random|RandomFloatinRange 5.0 15.0))
              (Audio|PlaySoundatLocation "/Game/MAIN/Pokemon/Sound/PokemonCriesAnime/ElectrodeCryExplode_Cue.ElectrodeCryExplode_Cue" _returnvalue "0, 0, 0" 1.0 1.0 0.0 0 0 0)
              (Utilities|FlowControl|Delay 2.0)
              (Effects|SpawnEmitteratLocation "/Game/FXs/3/Particles/P_ky_explosion.P_ky_explosion" _returnvalue "0, 0, 0" "10.000000,10.000000,10.000000")
              (Audio|PlaySoundatLocation "/Game/MAIN/Pokemon/Sound/Explosion_Cue.Explosion_Cue" _returnvalue "0, 0, 0" 1.0 1.0 0.0 0 0 0)
              (Rendering|SetVisibility (Variables|Character|GetMesh) false false)
              (Utilities|FlowControl|Delay 1.0)
              (Actor|DestroyActor))))))
    (:else)))

(fn ConstructionScript
  (|CallParentFunction))

(fn UseItem
  (|CallParentFunction)
  (bind _asmaster_character_bp (Utilities|Casting|CastToMasterCharacter_BP (Game|GetPlayerCharacter 0)))
  (Default|SummonPet _asmaster_character_bp "Electrode_BP_C")
  (return true))