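; Player fireball projectile that explodes on sphere overlap and damages NPCs.
; An NPC hit hides the fireball, subtracts random damage from the player character's Ability 1 range and turns the NPC hostile.
; A kill awards XP, stops the NPC's movement, marks it dead and notifies every quest in the quest log.
; The projectile destroys itself after a delay only on kills or non-NPC overlaps.
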(event OnComponentBeginOverlap(Sphere)
  (params (OverlappedComponent :type Primitive%20Component%20Object%20Reference) (OtherActor :type Actor%20Object%20Reference) (OtherComp :type Primitive%20Component%20Object%20Reference) (OtherBodyIndex :type Integer) (bFromSweep :type Boolean) (SweepResult :type Hit%20Result%20Structure%20%28by%20ref%29))
  (bind _output_get (Variables|Default|SetHitActor (.HitActor (Collision|BreakHitResult SweepResult))))
  (if (Utilities|ClassIsChildOf (Utilities|GetClass _output_get) "/Game/MAIN/Blueprints/NPC/NPC_Parent_BP.NPC_Parent_BP_C")
    (Effects|SpawnEmitteratLocation "/Game/FXs/2/AdvancedMagicFX13/Particles/P_ky_explosion1.P_ky_explosion1" (Transformation|GetActorLocation self) "0, 0, 0" "5.000000,5.000000,5.000000")
    (Rendering|SetVisibility (Variables|Default|GetFireball) false false)
    (bind _asnpc_parent_bp (Utilities|Casting|CastToNPC_Parent_BP (Variables|Default|GetHitActor)))
    (Variables|Default|SetNPC_Parent _asnpc_parent_bp)
    (bind _asmaster_character_bp (Utilities|Casting|CastToMasterCharacter_BP (Game|GetPlayerCharacter 0)))
    (bind _output_get_2 (Variables|/Game/MAIN/Blueprints/NPC/NPC_Parent_BP.NPC_Parent_BP_C|SetCurrentHealth (Variables|Default|GetNPC_Parent) (- (Variables|/Game/MAIN/Blueprints/NPC/NPC_Parent_BP.NPC_Parent_BP_C|GetCurrentHealth (Variables|Default|GetNPC_Parent)) (Math|Random|RandomIntegerinRange (Variables|/Game/MAIN/Blueprints/Player/MasterCharacter_BP.MasterCharacter_BP_C|GetAbility1FireballDamageMinAmount _asmaster_character_bp) (Variables|/Game/MAIN/Blueprints/Player/MasterCharacter_BP.MasterCharacter_BP_C|GetAbility1FireballDamageMaxAmount _asmaster_character_bp)))))
    (Variables|/Game/MAIN/Blueprints/NPC/NPC_Parent_BP.NPC_Parent_BP_C|SetIsHostile (Variables|Default|GetNPC_Parent) true)
    (if (< _output_get_2 1)
      (if (not (Variables|/Game/MAIN/Blueprints/NPC/NPC_Parent_BP.NPC_Parent_BP_C|GetIsDead (Variables|Default|GetNPC_Parent)))
        (Utilities|FlowControl|Sequence
          (:then_0
            (Default|AddXP _asmaster_character_bp 1e+01)
            (Components|Movement|StopMovementImmediately (Variables|/Script/Engine.Character|GetCharacterMovement (Variables|Default|GetNPC_Parent)))
            (Variables|/Script/Engine.CharacterMovementComponent|SetMaxWalkSpeed (Variables|/Script/Engine.Character|GetCharacterMovement (Variables|Default|GetNPC_Parent)) 0.0)
            (Pawn|Components|CharacterMovement|DisableMovement (Variables|/Script/Engine.Character|GetCharacterMovement (Variables|Default|GetNPC_Parent)))
            (Variables|/Game/MAIN/Blueprints/NPC/NPC_Parent_BP.NPC_Parent_BP_C|SetIsDead (Variables|Default|GetNPC_Parent) true)
            (Utilities|FlowControl|Delay 1.0)
            (Actor|DestroyActor))
          (:then_1
            (for _array_element (Variables|/Game/MAIN/QuestSystem/QuestLog.QuestLog_C|GetQuests (Variables|/Game/MAIN/Blueprints/Player/MasterCharacter_BP.MasterCharacter_BP_C|GetQuestLog _asmaster_character_bp))
              (Default|CallKilledEnemy _array_element (Variables|Default|GetNPC_Parent)))))))
    (else
      (Effects|SpawnEmitteratLocation "/Game/FXs/2/AdvancedMagicFX13/Particles/P_ky_explosion1.P_ky_explosion1" (Transformation|GetActorLocation self) "0, 0, 0" "5.000000,5.000000,5.000000")
      (Utilities|FlowControl|Delay 0.5)
      (Actor|DestroyActor))))

(fn ConstructionScript)