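; NPC_Turtle_BP is a turtle creature NPC Blueprint that shows its widget only when the player is nearby.
; Every tick, after calling the parent, it measures the distance to PlayerReference and toggles Widget0's visibility at a fixed range, without propagating to children.
; BeginPlay and overlap events are disabled stubs, and the construction script only calls the parent.
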(event EventBeginPlay
  (|CallParentFunction) ; This node is disabled and will not be called.\nDrag off pins to build functionality.
)

(event Collision|EventActorBeginOverlap
  (params (OtherActor :type Actor%20Object%20Reference))
  (|CallParentFunction OtherActor) ; This node is disabled and will not be called.\nDrag off pins to build functionality.
)

(event EventTick
  (params (DeltaSeconds :type Float%20%28single-precision%29))
  (bind _self self)
  (|CallParentFunction DeltaSeconds)
  (Utilities|IsValid _self
    (:Is%20Valid
      (if (<= (Transformation|GetDistanceTo _self (Variables|Default|GetPlayerReference)) 1e+03)
        (Rendering|SetVisibility (Variables|Default|GetWidget_0) true false)
        (else
          (Rendering|SetVisibility (Variables|Default|GetWidget_0) false false))))))

(fn ConstructionScript
  (|CallParentFunction))