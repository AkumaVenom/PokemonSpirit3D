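; Daemon spawner actor that keeps one NPC_Daemon_BP alive while the player is within a set radius.
; On BeginPlay it caches the first MasterCharacter_BP found as the player reference.
; Tick checks the distance and, if no valid daemon exists, spawns one at SpawnPoint with the configured scale, so a destroyed daemon is replaced.
; Its DoOnce resets on both branches, so the check effectively repeats every tick in range.
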(event EventBeginPlay
  (bind _outactors (Actor|GetAllActorsOfClass "/Game/MAIN/Blueprints/Player/MasterCharacter_BP.MasterCharacter_BP_C"))
  (Variables|Default|SetPlayerRef (Utilities|Array|Get(acopy) _outactors)))

(event Collision|EventActorBeginOverlap
  (params (OtherActor :type Actor%20Object%20Reference)))

(event EventTick
  (params (DeltaSeconds :type Float%20%28single-precision%29))
  (if (< (Transformation|GetDistanceTo self (Variables|Default|GetPlayerRef)) (Variables|Default|GetRadius))
    (Utilities|FlowControl|DoOnce false :!label _label
      (:Completed
        (Variables|Default|GetDaemon
          (:then
            (goto _label Reset))
          (:else
            (bind _returnvalue (AI|SpawnAIFromClass "/Game/MAIN/Blueprints/NPC/Creature/NPC_Daemon_BP.NPC_Daemon_BP_C" 0 (Transformation|GetWorldLocation (Variables|Default|GetSpawnPoint)) "0, 0, 0" true))
            (bind _output_get (Variables|Default|SetDaemon _returnvalue))
            (Transformation|SetActorScale3D _output_get (Variables|Default|GetNPC_Scale))
            (goto _label Reset)))))))

(fn ConstructionScript)