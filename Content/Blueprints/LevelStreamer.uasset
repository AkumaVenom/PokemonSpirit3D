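; LevelStreamer is a trigger actor that streams the level named by LevelToStream in and out as MasterCharacter_BP overlaps its boxes.
; LoadStreamBox loads the level without blocking and makes it visible, then sets IsMiddleLevelLoaded on the player character if the level reports as loaded.
; Four unload boxes share one path that unloads the same level without blocking.
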(event OnComponentBeginOverlap(LoadStreamBox)
  (params (OverlappedComponent :type Primitive%20Component%20Object%20Reference) (OtherActor :type Actor%20Object%20Reference) (OtherComp :type Primitive%20Component%20Object%20Reference) (OtherBodyIndex :type Integer) (bFromSweep :type Boolean) (SweepResult :type Hit%20Result%20Structure%20%28by%20ref%29))
  (bind _leveltostream (Variables|Default|GetLevelToStream))
  (Utilities|Casting|CastToMasterCharacter_BP OtherActor)
  (Game|LoadStreamLevel(byName) _leveltostream true)
  (if (Class|LevelStreaming|IsLevelLoaded (Class|GameplayStatics|GetStreamingLevel _leveltostream))
    (bind _asmaster_character_bp (Utilities|Casting|CastToMasterCharacter_BP (Game|GetPlayerCharacter 0)))
    (Variables|/Game/MAIN/Blueprints/Player/MasterCharacter_BP.MasterCharacter_BP_C|SetIsMiddleLevelLoaded _asmaster_character_bp true)))

(event OnComponentBeginOverlap(UnloadStreamBox)
  (params (OverlappedComponent :type Primitive%20Component%20Object%20Reference) (OtherActor :type Actor%20Object%20Reference) (OtherComp :type Primitive%20Component%20Object%20Reference) (OtherBodyIndex :type Integer) (bFromSweep :type Boolean) (SweepResult :type Hit%20Result%20Structure%20%28by%20ref%29))
  (Utilities|Casting|CastToMasterCharacter_BP OtherActor)
  (Game|UnloadStreamLevel(byName) (Variables|Default|GetLevelToStream) false))

(event OnComponentBeginOverlap(UnloadStreamBox2)
  (params (OverlappedComponent :type Primitive%20Component%20Object%20Reference) (OtherActor :type Actor%20Object%20Reference) (OtherComp :type Primitive%20Component%20Object%20Reference) (OtherBodyIndex :type Integer) (bFromSweep :type Boolean) (SweepResult :type Hit%20Result%20Structure%20%28by%20ref%29))
  (Utilities|Casting|CastToMasterCharacter_BP OtherActor)
  (Game|UnloadStreamLevel(byName) (Variables|Default|GetLevelToStream) false))

(event OnComponentBeginOverlap(UnloadStreamBox3)
  (params (OverlappedComponent :type Primitive%20Component%20Object%20Reference) (OtherActor :type Actor%20Object%20Reference) (OtherComp :type Primitive%20Component%20Object%20Reference) (OtherBodyIndex :type Integer) (bFromSweep :type Boolean) (SweepResult :type Hit%20Result%20Structure%20%28by%20ref%29))
  (Utilities|Casting|CastToMasterCharacter_BP OtherActor)
  (Game|UnloadStreamLevel(byName) (Variables|Default|GetLevelToStream) false))

(event OnComponentBeginOverlap(UnloadStreamBox4)
  (params (OverlappedComponent :type Primitive%20Component%20Object%20Reference) (OtherActor :type Actor%20Object%20Reference) (OtherComp :type Primitive%20Component%20Object%20Reference) (OtherBodyIndex :type Integer) (bFromSweep :type Boolean) (SweepResult :type Hit%20Result%20Structure%20%28by%20ref%29))
  (Utilities|Casting|CastToMasterCharacter_BP OtherActor)
  (Game|UnloadStreamLevel(byName) (Variables|Default|GetLevelToStream) false))

(event EventBeginPlay)

(event Collision|EventActorBeginOverlap
  (params (OtherActor :type Actor%20Object%20Reference)))

(fn ConstructionScript)