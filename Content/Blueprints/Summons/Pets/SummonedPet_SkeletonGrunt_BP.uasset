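; Summoned skeleton grunt pet Blueprint that holds the pet in place during a montage when it spawns.
; On BeginPlay, after the parent logic runs, it disables movement and plays a montage on the mesh.
; The montage's returned length drives a delay, after which movement switches back to Walking.
; Tick, overlap and construction add no logic of their own.
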(event EventBeginPlay
  (bind _charactermovement (Variables|Character|GetCharacterMovement))
  (|CallParentFunction)
  (Pawn|Components|CharacterMovement|DisableMovement _charactermovement)
  (bind _returnvalue (Animation|Montage|MontagePlay (Components|SkeletalMesh|GetAnimInstance (Variables|Character|GetMesh)) 0 1.0 "MontageLength" 0.0 true))
  (Utilities|FlowControl|Delay _returnvalue)
  (Pawn|Components|CharacterMovement|SetMovementMode _charactermovement "MOVE_Walking" 0))

(event Collision|EventActorBeginOverlap
  (params (OtherActor :type Actor%20Object%20Reference))
  (|CallParentFunction OtherActor) ; This node is disabled and will not be called.\nDrag off pins to build functionality.
)

(event EventTick
  (params (DeltaSeconds :type Float%20%28single-precision%29))
  (|CallParentFunction DeltaSeconds) ; This node is disabled and will not be called.\nDrag off pins to build functionality.
)

(fn ConstructionScript
  (|CallParentFunction))