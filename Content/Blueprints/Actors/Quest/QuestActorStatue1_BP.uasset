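; Quest interactable statue actor that advances StoryQuest_1 when the player interacts with it.
; Interact finds the first StoryQuest_1 actor and continues only if that quest is started and not complete.
; A DoOnce then reports the statue to the quest through CallInteracted and freezes the player's movement.
; After a fixed delay it runs DisplayTurnIn for the quest, then restores walking.
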(event EventBeginPlay)

(event Collision|EventActorBeginOverlap
  (params (OtherActor :type Actor%20Object%20Reference)))

(event EventTick
  (params (DeltaSeconds :type Float%20%28single-precision%29)))

(event EventInteract
  (params (Interacter :type Actor%20Object%20Reference))
  (bind _asmaster_character_bp (Utilities|Casting|CastToMasterCharacter_BP (Game|GetPlayerCharacter 0)))
  (bind _outactors (Actor|GetAllActorsOfClass "/Game/MAIN/QuestSystem/Quests/Story/StoryQuest_1.StoryQuest_1_C"))
  (if (Variables|/Game/MAIN/QuestSystem/Quests/QuestMaster_BP.QuestMaster_BP_C|GetIsQuestStarted (Utilities|Array|Get(acopy) _outactors))
    (if (not (Variables|/Game/MAIN/QuestSystem/Quests/QuestMaster_BP.QuestMaster_BP_C|GetIsComplete (Utilities|Array|Get(acopy) _outactors)))
      (Utilities|FlowControl|DoOnce false
        (:Completed
          (Default|CallInteracted (Utilities|Array|Get(acopy) _outactors) self)
          (Pawn|Components|CharacterMovement|DisableMovement (Variables|/Script/Engine.Character|GetCharacterMovement _asmaster_character_bp))
          (Components|Movement|StopMovementImmediately (Variables|/Script/Engine.Character|GetCharacterMovement _asmaster_character_bp))
          (Utilities|FlowControl|Delay 6.0)
          (Utilities|DisplayTurnin (Utilities|Array|Get(acopy) _outactors)
            (:Out
              (Pawn|Components|CharacterMovement|SetMovementMode (Variables|/Script/Engine.Character|GetCharacterMovement _asmaster_character_bp) "MOVE_Walking" 0))))))))

(fn ConstructionScript)