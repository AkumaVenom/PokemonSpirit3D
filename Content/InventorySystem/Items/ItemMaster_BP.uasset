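; Base pickup item for the inventory system, with a UseItem stub that returns false.
; Interact sets player flags for starter Pokeballs and restricts quest items to those whose class matches a quest objective target, unless the Pokeball is in use.
; PickupItem, gated by DoOnce, adds the item to the player's inventory component.
; On success it notifies incomplete quests and destroys the actor after a short delay.
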(event Custom|PickupItem
  (Utilities|FlowControl|DoOnce false
    (:Completed
      (bind _asmaster_character_bp (Utilities|Casting|CastToMasterCharacter_BP (Game|GetPlayerCharacter 0)))
      (bind _success (Default|AddtoInventory (Variables|/Game/MAIN/Blueprints/Player/MasterCharacter_BP.MasterCharacter_BP_C|GetInventoryComponent _asmaster_character_bp) (Utilities|Struct|MakeSlotStructure (Variables|Default|GetItemStructure) 1)))
      (if _success
        (Utilities|FlowControl|Sequence
          (:then_0
            (Utilities|FlowControl|Delay 0.2)
            (Utilities|IsValid self
              (:Is%20Valid
                (Actor|DestroyActor))))
          (:then_1
            (for _array_element (Variables|/Game/MAIN/QuestSystem/QuestLog.QuestLog_C|GetQuests (Variables|/Game/MAIN/Blueprints/Player/MasterCharacter_BP.MasterCharacter_BP_C|GetQuestLog _asmaster_character_bp))
              (if (not (Variables|/Game/MAIN/QuestSystem/Quests/QuestMaster_BP.QuestMaster_BP_C|GetIsComplete _array_element))
                (Default|CallCollectedItem _array_element self)))))))))

(event EventBeginPlay
  (bind _outactors (Actor|GetAllActorsOfClass "/Game/MAIN/Blueprints/Player/MasterCharacter_BP.MasterCharacter_BP_C"))
  (for _array_element _outactors
    (Variables|Default|SetPlayerReference _array_element)))

(event Collision|EventActorBeginOverlap
  (params (OtherActor :type Actor%20Object%20Reference))
  (if true
    _))

(event EventTick
  (params (DeltaSeconds :type Float%20%28single-precision%29))
  (if true
    _))

(event EventInteract
  (params (Interacter :type Actor%20Object%20Reference))
  (bind _playerreference (Variables|Default|GetPlayerReference)
    (:then
      (if (not (Variables|Default|GetIsPokeballInUse))
        (if (and (Variables|Default|GetIsStarterPokeball1) (not (Variables|/Game/MAIN/Blueprints/Player/MasterCharacter_BP.MasterCharacter_BP_C|GetPickedUpStarterPokeball1 _playerreference)))
          (bind _playerreference_2 (Variables|Default|GetPlayerReference)
            (:then
              (Variables|/Game/MAIN/Blueprints/Player/MasterCharacter_BP.MasterCharacter_BP_C|SetPickedUpStarterPokeball1 _playerreference_2 true)
              (CallFunction|PickupItem))
            (:else))
          (elif (and (Variables|Default|GetIsStarterPokeball2) (not (Variables|/Game/MAIN/Blueprints/Player/MasterCharacter_BP.MasterCharacter_BP_C|GetPickedUpStarterPokeball2 _playerreference)))
            (bind _playerreference_3 (Variables|Default|GetPlayerReference)
              (:then
                (Variables|/Game/MAIN/Blueprints/Player/MasterCharacter_BP.MasterCharacter_BP_C|SetPickedUpStarterPokeball2 _playerreference_3 true)
                (CallFunction|PickupItem))
              (:else))
            (elif (and (Variables|Default|GetIsStarterPokeball3) (not (Variables|/Game/MAIN/Blueprints/Player/MasterCharacter_BP.MasterCharacter_BP_C|GetPickedUpStarterPokeball3 _playerreference)))
              (bind _playerreference_4 (Variables|Default|GetPlayerReference)
                (:then
                  (Variables|/Game/MAIN/Blueprints/Player/MasterCharacter_BP.MasterCharacter_BP_C|SetPickedUpStarterPokeball3 _playerreference_4 true)
                  (CallFunction|PickupItem))
                (:else))
              (elif (and (Variables|Default|GetIsStarterPokeball4) (not (Variables|/Game/MAIN/Blueprints/Player/MasterCharacter_BP.MasterCharacter_BP_C|GetPickedUpStarterPokeball4 _playerreference)))
                (bind _playerreference_5 (Variables|Default|GetPlayerReference)
                  (:then
                    (Variables|/Game/MAIN/Blueprints/Player/MasterCharacter_BP.MasterCharacter_BP_C|SetPickedUpStarterPokeball4 _playerreference_5 true)
                    (CallFunction|PickupItem))
                  (:else))
                (elif (and (Variables|Default|GetIsStarterPokeball5) (not (Variables|/Game/MAIN/Blueprints/Player/MasterCharacter_BP.MasterCharacter_BP_C|GetPickedUpStarterPokeball5 _playerreference)))
                  (bind _playerreference_6 (Variables|Default|GetPlayerReference)
                    (:then
                      (Variables|/Game/MAIN/Blueprints/Player/MasterCharacter_BP.MasterCharacter_BP_C|SetPickedUpStarterPokeball5 _playerreference_6 true)
                      (CallFunction|PickupItem))
                    (:else))
                  (elif (.isquestitem (Variables|Default|GetItemStructure))
                    (bind _asmaster_character_bp (Utilities|Casting|CastToMasterCharacter_BP (Game|GetPlayerCharacter 0)))
                    (for _array_element (Variables|/Game/MAIN/QuestSystem/QuestLog.QuestLog_C|GetQuests (Variables|/Game/MAIN/Blueprints/Player/MasterCharacter_BP.MasterCharacter_BP_C|GetQuestLog _asmaster_character_bp))
                      (for _array_element_2 (Variables|/Game/MAIN/QuestSystem/Quests/QuestMaster_BP.QuestMaster_BP_C|GetObjectives _array_element)
                        (if (== (Utilities|GetClass (.Target (Utilities|Struct|BreakObjectiveData _array_element_2))) (Utilities|GetClass self))
                          (CallFunction|PickupItem))))
                    (else
                      (CallFunction|PickupItem))))))))))
    (:else)))

(fn ConstructionScript)

(fn UseItem
  (return false))