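; Quest actor that tracks an Objectives array for a story or side quest and displays matching quest and question-mark sprites.
; BeginPlay binds location, interaction, collection and kill events, with Check functions completing matching objectives and flagging UI updates.
; Tick rechecks collection objectives against the player's inventory, spawns or destroys markers at location and interaction targets, and gates the quest mark on a prerequisite.
; It also yaws itself toward the player camera, billboard-style.
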(event Custom|SetQuestMarkInvisible
  (Rendering|SetVisibility (Variables|Default|GetQuestMark) false false))

(event Custom|SetQuestionMark
  (if (Utilities|Enum|Equal(Enum) (Variables|Default|GetObjectiveType) "NewEnumerator0")
    (if (Variables|Default|GetIsStoryQuest)
      (Variables|Default|GetLocationStoryQuestionMark
        (:then)
        (:else
          (bind _returnvalue (Game|SpawnActorfromClass "/Game/MAIN/Blueprints/Actors/Quest/StoryQuestionMark_BP.StoryQuestionMark_BP_C" (Math|Transform|MakeTransform (Transformation|GetActorLocation (Variables|Default|GetObjectiveTarget)) "0, 0, 0" "1,1,1") "AlwaysSpawn" 0 0))
          (Variables|Default|SetLocationStoryQuestionMark _returnvalue)))
      (else
        (Variables|Default|GetLocationSideQuestionMark
          (:then)
          (:else
            (bind _returnvalue_2 (Game|SpawnActorfromClass "/Game/MAIN/Blueprints/Actors/Quest/SideQuestionMark_BP.SideQuestionMark_BP_C" (Math|Transform|MakeTransform (Transformation|GetActorLocation (Variables|Default|GetObjectiveTarget)) "0, 0, 0" "1,1,1") "AlwaysSpawn" 0 0))
            (Variables|Default|SetLocationSideQuestionMark _returnvalue_2)))))
    (elif (Utilities|Enum|Equal(Enum) (Variables|Default|GetObjectiveType) "NewEnumerator1")
      (if (Variables|Default|GetIsStoryQuest)
        (Variables|Default|GetInteractStoryQuestionMark
          (:then)
          (:else
            (bind _returnvalue_3 (Game|SpawnActorfromClass "/Game/MAIN/Blueprints/Actors/Quest/StoryQuestionMark_BP.StoryQuestionMark_BP_C" (Math|Transform|MakeTransform (Transformation|GetActorLocation (Variables|Default|GetObjectiveTarget)) "0, 0, 0" "1,1,1") "AlwaysSpawn" 0 0))
            (Variables|Default|SetInteractStoryQuestionMark _returnvalue_3)))
        (else
          (Variables|Default|GetInteractSideQuestionMark
            (:then)
            (:else
              (bind _returnvalue_4 (Game|SpawnActorfromClass "/Game/MAIN/Blueprints/Actors/Quest/SideQuestionMark_BP.SideQuestionMark_BP_C" (Math|Transform|MakeTransform (Transformation|GetActorLocation (Variables|Default|GetObjectiveTarget)) "0, 0, 0" "1,1,1") "AlwaysSpawn" 0 0))
              (Variables|Default|SetInteractSideQuestionMark _returnvalue_4))))))))

(event Custom|SetQuestionMarkInvisible
  (Rendering|SetVisibility (Variables|Default|GetQuestionMark) false false))

(event EventTick
  (params (DeltaSeconds :type Float%20%28single-precision%29))
  (bind _objectives (Variables|Default|GetObjectives))
  (bind _prerequisite (Variables|Default|GetPreRequisite))
  (bind _objectiveindexcollection (Variables|Default|GetObjectiveIndexCollection))
  (bind _objectives_2 (Variables|Default|GetObjectives))
  (bind _objectiveindexcollection_2 (Variables|Default|GetObjectiveIndexCollection))
  (bind _objectives_3 (Variables|Default|GetObjectives))
  (bind _objectiveindexcollection_3 (Variables|Default|GetObjectiveIndexCollection))
  (bind _output (Utilities|Array|Get(acopy) _objectives _objectiveindexcollection))
  (bind _output_2 (Utilities|Array|Get(acopy) _objectives_2 _objectiveindexcollection_2))
  (bind _output_3 (Utilities|Array|Get(acopy) _objectives_3 _objectiveindexcollection_3))
  (if (Variables|Default|GetIsComplete)
    (Utilities|FlowControl|DoOnce false
      (:Completed
        (Rendering|SetVisibility (Variables|Default|GetQuestMark) false false)))
    (else
      (Utilities|FlowControl|Sequence
        (:then_0
          (for _array_element (Variables|Default|GetObjectives)
            (Variables|Default|SetObjectiveType (.type _array_element))
            (Variables|Default|SetObjectiveTarget (.target _array_element))
            (Utilities|FlowControl|Sequence
              (:then_0
                (bind _playerinventory (Variables|Default|GetPlayerInventory)
                  (:then
                    (if (Utilities|Enum|Equal(Enum) (.type _array_element) "NewEnumerator2")
                      (if (.iscomplete _array_element)
                        (if (< (Variables|/Game/MAIN/InventorySystem/InventoryComponent.InventoryComponent_C|GetRunningTotal _playerinventory) (.number _array_element))
                          (Utilities|FlowControl|DoOnce false :!label _label
                            (:Completed
                              (Utilities|Array|SetArrayElem (Variables|Default|GetObjectives) (Variables|Default|GetObjectiveIndexCollection) (Utilities|Struct|MakeObjectiveData (.description _output) (.type _output) false (.target _output) (.number _output) (.killedenemyitemcolleced_tag _output)))))
                          (else
                            (Utilities|FlowControl|Sequence
                              (:then_0
                                (goto _label Reset))
                              (:then_1
                                (if (>= (.number _array_element) (Variables|/Game/MAIN/InventorySystem/InventoryComponent.InventoryComponent_C|GetRunningTotal _playerinventory)) :!label _label_2
                                  (Utilities|FlowControl|DoOnce false :!label _label_3
                                    (:Completed
                                      (Utilities|Array|SetArrayElem (Variables|Default|GetObjectives) (Variables|Default|GetObjectiveIndexCollection) (Utilities|Struct|MakeObjectiveData (.description _output_2) (.type _output_2) true (.target _output_2) (.number _output_2) (.killedenemyitemcolleced_tag _output_2)))))
                                  (else
                                    (goto _label_3 Reset)))))))
                        (elif (< (Variables|/Game/MAIN/InventorySystem/InventoryComponent.InventoryComponent_C|GetRunningTotal _playerinventory) (.number _array_element))
                          (Utilities|FlowControl|DoOnce false :!label _label_4
                            (:Completed
                              (Utilities|Array|SetArrayElem (Variables|Default|GetObjectives) (Variables|Default|GetObjectiveIndexCollection) (Utilities|Struct|MakeObjectiveData (.description _output_3) (.type _output_3) false (.target _output_3) (.number _output_3) (.killedenemyitemcolleced_tag _output_3)))))
                          (else
                            (Utilities|FlowControl|Sequence
                              (:then_0
                                (goto _label_2))
                              (:then_1
                                (goto _label_4 Reset))))))))
                  (:else)))
              (:then_1
                (CallFunction|SetQuestionMark)
                (if (.iscomplete _array_element)
                  (Utilities|FlowControl|Sequence
                    (:then_0
                      (if (Utilities|Enum|Equal(Enum) (.type _array_element) "NewEnumerator0")
                        (Utilities|FlowControl|Sequence
                          (:then_0
                            (bind _locationstoryquestionmark (Variables|Default|GetLocationStoryQuestionMark)
                              (:then
                                (Actor|DestroyActor _locationstoryquestionmark))
                              (:else)))
                          (:then_1
                            (bind _locationsidequestionmark (Variables|Default|GetLocationSideQuestionMark)
                              (:then
                                (Actor|DestroyActor _locationsidequestionmark))
                              (:else))))))
                    (:then_1
                      (if (Utilities|Enum|Equal(Enum) (.type _array_element) "NewEnumerator1")
                        (Utilities|FlowControl|Sequence
                          (:then_0
                            (bind _interactstoryquestionmark (Variables|Default|GetInteractStoryQuestionMark)
                              (:then
                                (Actor|DestroyActor _interactstoryquestionmark))
                              (:else)))
                          (:then_1
                            (bind _interactsidequestionmark (Variables|Default|GetInteractSideQuestionMark)
                              (:then
                                (Actor|DestroyActor _interactsidequestionmark))
                              (:else))))))))))))
        (:then_1
          (Utilities|FlowControl|Delay 0.02)
          (if (== _prerequisite 0)
            (Utilities|FlowControl|DoOnce false :!label _label_5
              (:Completed
                (Rendering|SetVisibility (Variables|Default|GetQuestMark) true false)))
            (elif (Variables|QuestMaster_BP_C|GetIsComplete _prerequisite)
              (goto _label_5))))
        (:then_2
          (Utilities|FlowControl|Delay 0.05)
          (Transformation|SetActorRotation (Math|Rotator|MakeRotator 0.0 0.0 (.yaw (Math|Rotator|FindLookatRotation (Transformation|GetWorldLocation (Variables|/Game/MAIN/Blueprints/Player/MasterCharacter_BP.MasterCharacter_BP_C|GetFollowCamera (Variables|Default|GetPlayerReference))) (Transformation|GetWorldLocation (Variables|Default|GetQuestMark)))))))
        (:then_3
          (if (Variables|Default|GetIsQuestStarted)
            (Utilities|FlowControl|Sequence
              (:then_0
                (bind _locationstoryquestionmark_2 (Variables|Default|GetLocationStoryQuestionMark)
                  (:then
                    (Rendering|SetVisibility (Variables|/Game/MAIN/Blueprints/Actors/Quest/StoryQuestionMark_BP.StoryQuestionMark_BP_C|GetQuestionMark _locationstoryquestionmark_2) true false))
                  (:else)))
              (:then_1
                (bind _interactstoryquestionmark_2 (Variables|Default|GetInteractStoryQuestionMark)
                  (:then
                    (Rendering|SetVisibility (Variables|/Game/MAIN/Blueprints/Actors/Quest/StoryQuestionMark_BP.StoryQuestionMark_BP_C|GetQuestionMark _interactstoryquestionmark_2) true false))
                  (:else))))))
        (:then_4
          (for _array_element_2 (Variables|Default|GetObjectives)
            (if (.iscomplete _array_element_2)
              (if (Variables|Default|GetIsQuestGiverTurnIn)
                (Rendering|SetVisibility (Variables|Default|GetQuestionMark) true false))
              (else
                (Rendering|SetVisibility (Variables|Default|GetQuestionMark) false false)))))))))

(event Collision|EventActorBeginOverlap
  (params (OtherActor :type Actor%20Object%20Reference)))

(event EventBeginPlay
  (Utilities|FlowControl|Sequence
    (:then_0
      (if (Variables|Default|GetIsStoryQuest)
        (Utilities|FlowControl|Sequence
          (:then_0
            (Rendering|Components|Sprite|SetSprite (Variables|Default|GetQuestionMark) "/Game/Assets/Effects/Texture/StoryQuestionMark.StoryQuestionMark"))
          (:then_1
            (Rendering|Components|Sprite|SetSprite (Variables|Default|GetQuestMark) "/Game/Assets/Effects/Texture/StoryQuestMark.StoryQuestMark")))
        (else
          (Utilities|FlowControl|Sequence
            (:then_0
              (Rendering|Components|Sprite|SetSprite (Variables|Default|GetQuestionMark) "/Game/Assets/Effects/Texture/SideQuestionMark.SideQuestionMark"))
            (:then_1
              (Rendering|Components|Sprite|SetSprite (Variables|Default|GetQuestMark) "/Game/Assets/Effects/Texture/SideQuestMark.SideQuestMark"))))))
    (:then_1
      (bind _asmaster_character_bp (Utilities|Casting|CastToMasterCharacter_BP (Game|GetPlayerCharacter 0)))
      (bind _output_get (Variables|Default|SetPlayerReference _asmaster_character_bp))
      (Variables|Default|SetPlayerInventory (Variables|/Game/MAIN/Blueprints/Player/MasterCharacter_BP.MasterCharacter_BP_C|GetInventoryComponent _output_get))
      (EventDispatchers|BindEventtoLocationReached (EventDispatchers|CreateEvent :!event CheckLocationObjective))
      (EventDispatchers|BindEventtoInteracted (EventDispatchers|CreateEvent :!event CheckInteractionObjective))
      (EventDispatchers|BindEventtoCollectedItem (EventDispatchers|CreateEvent :!event CheckCollectionObjective))
      (EventDispatchers|BindEventtoKilledEnemy (EventDispatchers|CreateEvent :!event CheckKilledEnemy)))))

(fn ConstructionScript)

(fn OrganiseQuestinEditor
  (Transformation|SetActorLocation (Transformation|GetActorLocation (Actor|GetAttachParentActor)) false false))

(fn CheckLocationObjective
  (params (LocationReached :type Location%20Marker%20Object%20Reference))
  (for (_array_element _array_index) (Variables|Default|GetObjectives)
    (bind _output_get (Variables|Default|SetObjectiveIndexLocation _array_index))
    (Variables|Default|SetObjectiveWaypointIndex _output_get)
    (if (and (not (.IsComplete (Utilities|Struct|BreakObjectiveData _array_element))) (== (.Target (Utilities|Struct|BreakObjectiveData _array_element)) LocationReached))
      (Utilities|Array|SetArrayElem (Variables|Default|GetObjectives) (Variables|Default|GetObjectiveIndexLocation) (Utilities|Struct|MakeObjectiveData (.description (Utilities|Array|Get(acopy) (Variables|Default|GetObjectives) (Variables|Default|GetObjectiveIndexLocation))) (.type (Utilities|Array|Get(acopy) (Variables|Default|GetObjectives) (Variables|Default|GetObjectiveIndexLocation))) true (.target (Utilities|Array|Get(acopy) (Variables|Default|GetObjectives) (Variables|Default|GetObjectiveIndexLocation))) (.number (Utilities|Array|Get(acopy) (Variables|Default|GetObjectives) (Variables|Default|GetObjectiveIndexLocation)))))
      (LocalVariables|SetUpdateUI true))))

(fn CheckInteractionObjective
  (params (InteractionTarget :type Actor%20Object%20Reference))
  (for (_array_element _array_index) (Variables|Default|GetObjectives)
    (bind _output_get (Variables|Default|SetObjectiveIndexInteration _array_index))
    (Variables|Default|SetObjectiveWaypointIndex _output_get)
    (if (and (not (.IsComplete (Utilities|Struct|BreakObjectiveData _array_element))) (== (.Target (Utilities|Struct|BreakObjectiveData _array_element)) InteractionTarget))
      (Utilities|Array|SetArrayElem (Variables|Default|GetObjectives) (Variables|Default|GetObjectiveIndexInteration) (Utilities|Struct|MakeObjectiveData (.description (Utilities|Array|Get(acopy) (Variables|Default|GetObjectives) (Variables|Default|GetObjectiveIndexInteration))) (.type (Utilities|Array|Get(acopy) (Variables|Default|GetObjectives) (Variables|Default|GetObjectiveIndexInteration))) true (.target (Utilities|Array|Get(acopy) (Variables|Default|GetObjectives) (Variables|Default|GetObjectiveIndexInteration))) (.number (Utilities|Array|Get(acopy) (Variables|Default|GetObjectives) (Variables|Default|GetObjectiveIndexInteration)))))
      (LocalVariables|SetUpdateUI true))))

(fn CheckCollectionObjective
  (params (Item :type Item%20Master%20BP%20Object%20Reference))
  (for (_array_element _array_index) (Variables|Default|GetObjectives)
    (bind _output_get (Variables|Default|SetObjectiveIndexCollection _array_index))
    (Variables|Default|SetObjectiveWaypointIndex _output_get)
    (if (not (.IsComplete (Utilities|Struct|BreakObjectiveData _array_element)))
      (if (Utilities|Name|Equal(Name) (.KilledEnemyItemColleced_Tag (Utilities|Struct|BreakObjectiveData _array_element)) (Variables|/Game/MAIN/InventorySystem/Items/ItemMaster_BP.ItemMaster_BP_C|GetTag Item))
        (bind _isininventory (Default|InventoryQuery (Variables|Default|GetPlayerInventory) (Utilities|GetClass Item) (.Number (Utilities|Struct|BreakObjectiveData _array_element))))
        (if _isininventory
          (Utilities|Array|SetArrayElem (Variables|Default|GetObjectives) (Variables|Default|GetObjectiveIndexCollection) (Utilities|Struct|MakeObjectiveData (.description (Utilities|Array|Get(acopy) (Variables|Default|GetObjectives) (Variables|Default|GetObjectiveIndexCollection))) (.type (Utilities|Array|Get(acopy) (Variables|Default|GetObjectives) (Variables|Default|GetObjectiveIndexCollection))) true (.target (Utilities|Array|Get(acopy) (Variables|Default|GetObjectives) (Variables|Default|GetObjectiveIndexCollection))) (.number (Utilities|Array|Get(acopy) (Variables|Default|GetObjectives) (Variables|Default|GetObjectiveIndexCollection))) (.killedenemyitemcolleced_tag (Utilities|Array|Get(acopy) (Variables|Default|GetObjectives) (Variables|Default|GetObjectiveIndexCollection)))))
          (LocalVariables|SetUpdateUI true))))))

(fn CheckKilledEnemy
  (params (Enemy :type NPC%20Parent%20BP%20Object%20Reference))
  (for (_array_element _array_index) (Variables|Default|GetObjectives)
    (bind _output_get (Variables|Default|SetObjectiveIndexKill _array_index))
    (Variables|Default|SetObjectiveWaypointIndex _output_get)
    (if (Utilities|Name|Equal(Name) (.KilledEnemyItemColleced_Tag (Utilities|Struct|BreakObjectiveData _array_element)) (Variables|/Game/MAIN/Blueprints/NPC/NPC_Parent_BP.NPC_Parent_BP_C|GetTag Enemy))
      (bind _result (Math|Integer|IncrementInt (Variables|Default|GetCurrentKillCount))
        (:%20%20
          (if (>= _result (.Number (Utilities|Struct|BreakObjectiveData _array_element)))
            (Utilities|Array|SetArrayElem (Variables|Default|GetObjectives) (Variables|Default|GetObjectiveIndexKill) (Utilities|Struct|MakeObjectiveData (.description (Utilities|Array|Get(acopy) (Variables|Default|GetObjectives) (Variables|Default|GetObjectiveIndexKill))) (.type (Utilities|Array|Get(acopy) (Variables|Default|GetObjectives) (Variables|Default|GetObjectiveIndexKill))) true (.target (Utilities|Array|Get(acopy) (Variables|Default|GetObjectives) (Variables|Default|GetObjectiveIndexKill))) (.number (Utilities|Array|Get(acopy) (Variables|Default|GetObjectives) (Variables|Default|GetObjectiveIndexKill)))))
            (LocalVariables|SetUpdateUI true)))))))

(fn IsQuestComplete
  (for _array_element (Variables|Default|GetObjectives)
    (if (not (.iscomplete _array_element))
      (Variables|Default|SetAllObjectivesComplete false)))
  (return (Variables|Default|GetAllObjectivesComplete)))