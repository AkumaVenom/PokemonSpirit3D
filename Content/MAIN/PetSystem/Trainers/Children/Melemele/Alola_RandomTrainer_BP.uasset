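; Random Alola trainer variant that picks its look at spawn and toggles mesh visibility by player proximity.
; BeginPlay rolls nested coin flips to choose a skeletal mesh and matching AnimBP, correcting roll for some meshes, and caches the player as a pet if PlayerReference is invalid.
; Tick compares distance to Radius through DoOnce gates: within range shows the mesh, out of range hides it only for the PlayerReference path, not the pet path.
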(event EventBeginPlay
  (|CallParentFunction)
  (CallFunction|SetRandomPedestrianMesh)
  (Variables|Default|GetPlayerReference
    (:then)
    (:else
      (bind _aspet_parent_bp (Utilities|Casting|CastToPet_Parent_BP (Game|GetPlayerCharacter 0)))
      (Variables|Default|SetPlayerAsPet _aspet_parent_bp))))

(event Collision|EventActorBeginOverlap
  (params (OtherActor :type Actor%20Object%20Reference))
  (|CallParentFunction OtherActor) ; This node is disabled and will not be called.\nDrag off pins to build functionality.
)

(event EventTick
  (params (DeltaSeconds :type Float%20%28single-precision%29))
  (bind _self self)
  (bind _self_2 self)
  (|CallParentFunction DeltaSeconds)
  (bind _playeraspet (Variables|Default|GetPlayerAsPet)
    (:then
      (Utilities|IsValid _self_2
        (:Is%20Valid
          (if (< (Transformation|GetDistanceTo _self_2 _playeraspet) (Variables|Default|GetRadius))
            (Utilities|FlowControl|DoOnce false :!label _label
              (:Completed
                (bind _mesh (Variables|Character|GetMesh :!label _label_2)
                  (:then
                    (Rendering|SetVisibility _mesh true false))
                  (:else))))
            (else
              (goto _label Reset))))))
    (:else
      (bind _playerreference (Variables|Default|GetPlayerReference)
        (:then
          (Utilities|IsValid _self
            (:Is%20Valid
              (if (< (Transformation|GetDistanceTo _self _playerreference) (Variables|Default|GetRadius))
                (Utilities|FlowControl|Sequence
                  (:then_0
                    (Utilities|FlowControl|DoOnce false :!label _label_3
                      (:Completed
                        (goto _label_2))))
                  (:then_1
                    (goto _label_4 Reset)))
                (else
                  (Utilities|FlowControl|Sequence
                    (:then_0
                      (Utilities|FlowControl|DoOnce false :!label _label_4
                        (:Completed
                          (bind _mesh_2 (Variables|Character|GetMesh)
                            (:then
                              (Rendering|SetVisibility _mesh_2 false false))
                            (:else)))))
                    (:then_1
                      (goto _label_3 Reset))))))))
        (:else)))))

(fn ConstructionScript
  (|CallParentFunction))

(fn SetRandomPedestrianMesh
  (bind _mesh (Variables|Character|GetMesh))
  (bind _mesh_2 (Variables|Character|GetMesh))
  (bind _mesh_3 (Variables|Character|GetMesh))
  (bind _mesh_4 (Variables|Character|GetMesh))
  (bind _mesh_5 (Variables|Character|GetMesh))
  (bind _mesh_6 (Variables|Character|GetMesh))
  (bind _mesh_7 (Variables|Character|GetMesh))
  (bind _returnvalue (Transformation|GetRelativeTransform _mesh))
  (bind _returnvalue_2 (Transformation|GetRelativeTransform _mesh_2))
  (bind _returnvalue_3 (Transformation|GetRelativeTransform _mesh_5))
  (bind _returnvalue_4 (Transformation|GetRelativeTransform _mesh_6))
  (bind _returnvalue_5 (Transformation|GetRelativeTransform _mesh_7))
  (if (Math|Random|RandomBoolwithWeight 0.5)
    (if (Math|Random|RandomBoolwithWeight 0.5)
      (if (Math|Random|RandomBoolwithWeight 0.5)
        (Class|SkinnedMeshComponent|SetSkeletalMesh _mesh_3 "/Game/MAIN/Pokemon/Trainers/680/680.680" true)
        (Class|SkeletalMeshComponent|SetAnimClass _mesh_3 "/Game/MAIN/Pokemon/Trainers/680/SummerMaleAnimBP.SummerMaleAnimBP_C")
        (else
          (Class|SkinnedMeshComponent|SetSkeletalMesh _mesh "/Game/MAIN/Pokemon/Trainers/Female2/677.677" true)
          (Class|SkeletalMeshComponent|SetAnimClass _mesh "/Game/MAIN/Pokemon/Trainers/Female2/TrainerFemale2AnimBP.TrainerFemale2AnimBP_C")
          (Transformation|SetRelativeRotation _mesh (Math|Rotator|MakeRotator 0.0 (.pitch (.rotation _returnvalue)) (.yaw (.rotation _returnvalue))) false false)))
      (elif (Math|Random|RandomBoolwithWeight 0.5)
        (Class|SkinnedMeshComponent|SetSkeletalMesh _mesh_7 "/Game/MAIN/Pokemon/Trainers/Male02/Male02.Male02" true)
        (Class|SkeletalMeshComponent|SetAnimClass _mesh_7 "/Game/MAIN/Pokemon/Trainers/Male02/Male02AnimBP.Male02AnimBP_C")
        (Transformation|SetRelativeRotation _mesh_7 (Math|Rotator|MakeRotator 9e+01 (.pitch (.rotation _returnvalue_5)) (.yaw (.rotation _returnvalue_5))) false false)
        (else
          (Class|SkinnedMeshComponent|SetSkeletalMesh _mesh_6 "/Game/MAIN/Pokemon/Trainers/Female3/679.679" true)
          (Class|SkeletalMeshComponent|SetAnimClass _mesh_6 "/Game/MAIN/Pokemon/Trainers/Female3/TrainerFemale3AnimBP.TrainerFemale3AnimBP_C")
          (Transformation|SetRelativeRotation _mesh_6 (Math|Rotator|MakeRotator 0.0 (.pitch (.rotation _returnvalue_4)) (.yaw (.rotation _returnvalue_4))) false false))))
    (elif (Math|Random|RandomBoolwithWeight 0.5)
      (if (Math|Random|RandomBoolwithWeight 0.5)
        (Class|SkinnedMeshComponent|SetSkeletalMesh _mesh_4 "/Game/MAIN/Pokemon/Trainers/Male01/689.689" true)
        (Class|SkeletalMeshComponent|SetAnimClass _mesh_4 "/Game/MAIN/Pokemon/Trainers/Male01/Male01AnimBP.Male01AnimBP_C")
        (else
          (Class|SkinnedMeshComponent|SetSkeletalMesh _mesh_2 "/Game/MAIN/Pokemon/Trainers/Male05/Male05.Male05" true)
          (Class|SkeletalMeshComponent|SetAnimClass _mesh_2 "/Game/MAIN/Pokemon/Trainers/Male05/Male05AnimBP.Male05AnimBP_C")
          (Transformation|SetRelativeRotation _mesh_2 (Math|Rotator|MakeRotator 9e+01 (.pitch (.rotation _returnvalue_2)) (.yaw (.rotation _returnvalue_2))) false false)))
      (else
        (Class|SkinnedMeshComponent|SetSkeletalMesh _mesh_5 "/Game/MAIN/Pokemon/Trainers/Female4/682.682" true)
        (Class|SkeletalMeshComponent|SetAnimClass _mesh_5 "/Game/MAIN/Pokemon/Trainers/Female4/TrainerFemale4AnimBP.TrainerFemale4AnimBP_C")
        (Transformation|SetRelativeRotation _mesh_5 (Math|Rotator|MakeRotator 0.0 (.pitch (.rotation _returnvalue_3)) (.yaw (.rotation _returnvalue_3))) false false))))
  (return))