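; Professor Oak NPC Blueprint that shows dialogue UI when a player character interacts with it.
; Interact casts the interacter to MasterCharacter_BP, has it calculate Oak's text, waits briefly, then toggles the ProfOak_UI widget on or off.
; A RemoveOaksUI event also closes the widget if it is open.
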(event Custom|RemoveOaksUI
  (bind _oakstextui (Variables|Default|GetOaksTextUI)
    (:then
      (Widget|RemovefromParent _oakstextui)
      (Variables|Default|SetOaksTextUI 0))
    (:else)))

(event EventBeginPlay
  (|CallParentFunction) ; This node is disabled and will not be called.\nDrag off pins to build functionality.
)

(event Collision|EventActorBeginOverlap
  (params (OtherActor :type Actor%20Object%20Reference))
  (|CallParentFunction OtherActor) ; This node is disabled and will not be called.\nDrag off pins to build functionality.
)

(event EventTick
  (params (DeltaSeconds :type Float%20%28single-precision%29))
  (|CallParentFunction DeltaSeconds) ; This node is disabled and will not be called.\nDrag off pins to build functionality.
)

(event EventInteract
  (params (Interacter :type Actor%20Object%20Reference))
  (bind _asmaster_character_bp (Utilities|Casting|CastToMasterCharacter_BP Interacter))
  (Default|CalculateProfessorOaksText _asmaster_character_bp)
  (Utilities|FlowControl|Delay 0.05)
  (bind _oakstextui (Variables|Default|GetOaksTextUI)
    (:then
      (Widget|RemovefromParent _oakstextui)
      (Variables|Default|SetOaksTextUI 0))
    (:else
      (bind _returnvalue (UserInterface|CreateWidget "/Game/MAIN/Pokemon/UI/ProfOak_UI.ProfOak_UI_C"))
      (bind _output_get (Variables|Default|SetOaksTextUI _returnvalue))
      (UserInterface|Viewport|AddtoViewport _output_get 0))))

(fn ConstructionScript
  (|CallParentFunction))