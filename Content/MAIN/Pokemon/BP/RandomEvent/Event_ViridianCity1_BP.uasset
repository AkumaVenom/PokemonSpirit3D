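; Random world event for Viridian City that can spawn a swarm of ten Voltorbs when the player character enters its trigger.
; CollisionEvent overlap has a 20% chance to start it, playing sound and flash, showing a UI widget and spawning AI at scene points.
; Cleanup destroys them and clears the started flag, either on leaving the Sphere or after a four-minute delay armed from Tick through a resettable DoOnce.
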(event OnComponentBeginOverlap(CollisionEvent)
  (params (OverlappedComponent :type Primitive%20Component%20Object%20Reference) (OtherActor :type Actor%20Object%20Reference) (OtherComp :type Primitive%20Component%20Object%20Reference) (OtherBodyIndex :type Integer) (bFromSweep :type Boolean) (SweepResult :type Hit%20Result%20Structure%20%28by%20ref%29))
  (Utilities|Casting|CastToMasterCharacter_BP OtherActor)
  (if (not (Math|Random|RandomBoolwithWeight 0.8))
    (if (not (Variables|Default|GetHasEventStarted))
      (Variables|Default|SetHasEventStarted true)
      (Audio|PlaySound2D "/Game/MAIN/Pokemon/Sound/EventSound_Cue.EventSound_Cue" 1.0 1.0 0.0 0 0)
      (Effects|SpawnEmitteratLocation "/Game/FXs/2/AdvancedMagicFX13/Particles/P_ky_flash2.P_ky_flash2" (Transformation|GetWorldLocation (Variables|Default|GetFlashPoint)) "0, 0, 0" "500.000000,500.000000,500.000000")
      (CallFunction|EventWidget)
      (bind _returnvalue (AI|SpawnAIFromClass "/Game/MAIN/PetSystem/Pets/Pokemon/Voltorb_BP.Voltorb_BP_C" 0 (Transformation|GetWorldLocation (Variables|Default|GetScene)) (Math|Rotator|MakeRotator 0.0 0.0 (Math|Random|RandomFloatinRange -1.8e+02 1.8e+02)) false 0))
      (Variables|Default|SetVoltorb1 _returnvalue)
      (bind _returnvalue_2 (AI|SpawnAIFromClass "/Game/MAIN/PetSystem/Pets/Pokemon/Voltorb_BP.Voltorb_BP_C" 0 (Transformation|GetWorldLocation (Variables|Default|GetScene1)) (Math|Rotator|MakeRotator 0.0 0.0 (Math|Random|RandomFloatinRange -1.8e+02 1.8e+02)) false 0))
      (Variables|Default|SetVoltorb2 _returnvalue_2)
      (bind _returnvalue_3 (AI|SpawnAIFromClass "/Game/MAIN/PetSystem/Pets/Pokemon/Voltorb_BP.Voltorb_BP_C" 0 (Transformation|GetWorldLocation (Variables|Default|GetScene2)) (Math|Rotator|MakeRotator 0.0 0.0 (Math|Random|RandomFloatinRange -1.8e+02 1.8e+02)) false 0))
      (Variables|Default|SetVoltorb3 _returnvalue_3)
      (bind _returnvalue_4 (AI|SpawnAIFromClass "/Game/MAIN/PetSystem/Pets/Pokemon/Voltorb_BP.Voltorb_BP_C" 0 (Transformation|GetWorldLocation (Variables|Default|GetScene3)) (Math|Rotator|MakeRotator 0.0 0.0 (Math|Random|RandomFloatinRange -1.8e+02 1.8e+02)) false 0))
      (Variables|Default|SetVoltorb4 _returnvalue_4)
      (bind _returnvalue_5 (AI|SpawnAIFromClass "/Game/MAIN/PetSystem/Pets/Pokemon/Voltorb_BP.Voltorb_BP_C" 0 (Transformation|GetWorldLocation (Variables|Default|GetScene4)) (Math|Rotator|MakeRotator 0.0 0.0 (Math|Random|RandomFloatinRange -1.8e+02 1.8e+02)) false 0))
      (Variables|Default|SetVoltorb5 _returnvalue_5)
      (bind _returnvalue_6 (AI|SpawnAIFromClass "/Game/MAIN/PetSystem/Pets/Pokemon/Voltorb_BP.Voltorb_BP_C" 0 (Transformation|GetWorldLocation (Variables|Default|GetScene5)) (Math|Rotator|MakeRotator 0.0 0.0 (Math|Random|RandomFloatinRange -1.8e+02 1.8e+02)) false 0))
      (Variables|Default|SetVoltorb6 _returnvalue_6)
      (bind _returnvalue_7 (AI|SpawnAIFromClass "/Game/MAIN/PetSystem/Pets/Pokemon/Voltorb_BP.Voltorb_BP_C" 0 (Transformation|GetWorldLocation (Variables|Default|GetScene6)) (Math|Rotator|MakeRotator 0.0 0.0 (Math|Random|RandomFloatinRange -1.8e+02 1.8e+02)) false 0))
      (Variables|Default|SetVoltorb7 _returnvalue_7)
      (bind _returnvalue_8 (AI|SpawnAIFromClass "/Game/MAIN/PetSystem/Pets/Pokemon/Voltorb_BP.Voltorb_BP_C" 0 (Transformation|GetWorldLocation (Variables|Default|GetScene7)) (Math|Rotator|MakeRotator 0.0 0.0 (Math|Random|RandomFloatinRange -1.8e+02 1.8e+02)) false 0))
      (Variables|Default|SetVoltorb8 _returnvalue_8)
      (bind _returnvalue_9 (AI|SpawnAIFromClass "/Game/MAIN/PetSystem/Pets/Pokemon/Voltorb_BP.Voltorb_BP_C" 0 (Transformation|GetWorldLocation (Variables|Default|GetScene8)) (Math|Rotator|MakeRotator 0.0 0.0 (Math|Random|RandomFloatinRange -1.8e+02 1.8e+02)) false 0))
      (Variables|Default|SetVoltorb9 _returnvalue_9)
      (bind _returnvalue_10 (AI|SpawnAIFromClass "/Game/MAIN/PetSystem/Pets/Pokemon/Voltorb_BP.Voltorb_BP_C" 0 (Transformation|GetWorldLocation (Variables|Default|GetScene9)) (Math|Rotator|MakeRotator 0.0 0.0 (Math|Random|RandomFloatinRange -1.8e+02 1.8e+02)) false 0))
      (Variables|Default|SetVoltorb10 _returnvalue_10))))

(event OnComponentEndOverlap(Sphere)
  (params (OverlappedComponent :type Primitive%20Component%20Object%20Reference) (OtherActor :type Actor%20Object%20Reference) (OtherComp :type Primitive%20Component%20Object%20Reference) (OtherBodyIndex :type Integer))
  (Utilities|Casting|CastToMasterCharacter_BP OtherActor)
  (CallFunction|CleanupEvent))

(event Custom|ResetEventCleanup
  (Utilities|FlowControl|DoOnce false) ; enters at Reset
)

(event Custom|CleanupEvent
  (Variables|Default|SetHasEventStarted false)
  (CallFunction|ResetEventCleanup)
  (bind _voltorb1 (Variables|Default|GetVoltorb1)
    (:then
      (Actor|DestroyActor _voltorb1))
    (:else
      _))
  (bind _voltorb2 (Variables|Default|GetVoltorb2)
    (:then
      (Actor|DestroyActor _voltorb2))
    (:else
      _))
  (bind _voltorb3 (Variables|Default|GetVoltorb3)
    (:then
      (Actor|DestroyActor _voltorb3))
    (:else
      _))
  (bind _voltorb4 (Variables|Default|GetVoltorb4)
    (:then
      (Actor|DestroyActor _voltorb4))
    (:else
      _))
  (bind _voltorb5 (Variables|Default|GetVoltorb5)
    (:then
      (Actor|DestroyActor _voltorb5))
    (:else
      _))
  (bind _voltorb6 (Variables|Default|GetVoltorb6)
    (:then
      (Actor|DestroyActor _voltorb6))
    (:else
      _))
  (bind _voltorb7 (Variables|Default|GetVoltorb7)
    (:then
      (Actor|DestroyActor _voltorb7))
    (:else
      _))
  (bind _voltorb8 (Variables|Default|GetVoltorb8)
    (:then
      (Actor|DestroyActor _voltorb8))
    (:else
      _))
  (bind _voltorb9 (Variables|Default|GetVoltorb9)
    (:then
      (Actor|DestroyActor _voltorb9))
    (:else
      _))
  (bind _voltorb10 (Variables|Default|GetVoltorb10)
    (:then
      (Actor|DestroyActor _voltorb10))
    (:else)))

(event EventBeginPlay)

(event Collision|EventActorBeginOverlap
  (params (OtherActor :type Actor%20Object%20Reference)))

(event EventTick
  (params (DeltaSeconds :type Float%20%28single-precision%29))
  (if (Variables|Default|GetHasEventStarted)
    (Utilities|FlowControl|DoOnce false
      (:Completed
        (Utilities|FlowControl|Delay 2.4e+02)
        (Variables|Default|SetHasEventStarted false)
        (CallFunction|ResetEventCleanup)
        (bind _voltorb1 (Variables|Default|GetVoltorb1)
          (:then
            (Actor|DestroyActor _voltorb1))
          (:else
            _))
        (bind _voltorb2 (Variables|Default|GetVoltorb2)
          (:then
            (Actor|DestroyActor _voltorb2))
          (:else
            _))
        (bind _voltorb3 (Variables|Default|GetVoltorb3)
          (:then
            (Actor|DestroyActor _voltorb3))
          (:else
            _))
        (bind _voltorb4 (Variables|Default|GetVoltorb4)
          (:then
            (Actor|DestroyActor _voltorb4))
          (:else
            _))
        (bind _voltorb5 (Variables|Default|GetVoltorb5)
          (:then
            (Actor|DestroyActor _voltorb5))
          (:else
            _))
        (bind _voltorb6 (Variables|Default|GetVoltorb6)
          (:then
            (Actor|DestroyActor _voltorb6))
          (:else
            _))
        (bind _voltorb7 (Variables|Default|GetVoltorb7)
          (:then
            (Actor|DestroyActor _voltorb7))
          (:else
            _))
        (bind _voltorb8 (Variables|Default|GetVoltorb8)
          (:then
            (Actor|DestroyActor _voltorb8))
          (:else
            _))
        (bind _voltorb9 (Variables|Default|GetVoltorb9)
          (:then
            (Actor|DestroyActor _voltorb9))
          (:else
            _))
        (bind _voltorb10 (Variables|Default|GetVoltorb10)
          (:then
            (Actor|DestroyActor _voltorb10))
          (:else))))))

(fn ConstructionScript)

(fn EventWidget
  (bind _returnvalue (UserInterface|CreateWidget "/Game/MAIN/Pokemon/UI/Event_ViridianCity1_UI.Event_ViridianCity1_UI_C"))
  (UserInterface|Viewport|AddtoViewport _returnvalue 0)
  (return))