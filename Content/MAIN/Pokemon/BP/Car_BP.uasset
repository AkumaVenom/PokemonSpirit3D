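; Car actor that gives itself a random body color and hides its mesh when far from the player.
; On BeginPlay, SetColor picks one of seven body material instances through nested coin flips with uneven odds, then a MasterCharacter_BP player reference is cached.
; Tick checks player distance against a fixed threshold, using two DoOnce nodes that reset each other so visibility changes only on crossing it.
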(event EventBeginPlay
  (CallFunction|SetColor)
  (bind _asmaster_character_bp (Utilities|Casting|CastToMasterCharacter_BP (Game|GetPlayerCharacter 0)))
  (Variables|Default|SetPlayerReference _asmaster_character_bp))

(event Collision|EventActorBeginOverlap
  (params (OtherActor :type Actor%20Object%20Reference)))

(event EventTick
  (params (DeltaSeconds :type Float%20%28single-precision%29))
  (bind _skeletalmesh (Variables|Default|GetSkeletalMesh))
  (bind _playerreference (Variables|Default|GetPlayerReference)
    (:then
      (if (> (Transformation|GetDistanceTo _playerreference) 2e+04)
        (Utilities|FlowControl|DoOnce false :!label _label
          (:Completed
            (Rendering|SetVisibility _skeletalmesh false false)
            (goto _label_2 Reset)))
        (else
          (Utilities|FlowControl|DoOnce false :!label _label_2
            (:Completed
              (Rendering|SetVisibility _skeletalmesh true false)
              (goto _label Reset))))))
    (:else)))

(fn ConstructionScript)

(fn SetColor
  (if (Math|Random|RandomBoolwithWeight 0.5)
    (if (Math|Random|RandomBoolwithWeight 0.5)
      (if (Math|Random|RandomBoolwithWeight 0.5)
        (Rendering|Material|SetMaterial (Variables|Default|GetSkeletalMesh) 2 "/Game/MAIN/Pokemon/Cars/Mini/PokeCarBody_M_Inst.PokeCarBody_M_Inst")
        (else
          (Rendering|Material|SetMaterial (Variables|Default|GetSkeletalMesh) 2 "/Game/MAIN/Pokemon/Cars/Mini/PokeCarBody_M_Inst1.PokeCarBody_M_Inst1")))
      (elif (Math|Random|RandomBoolwithWeight 0.5)
        (Rendering|Material|SetMaterial (Variables|Default|GetSkeletalMesh) 2 "/Game/MAIN/Pokemon/Cars/Mini/PokeCarBody_M_Inst2.PokeCarBody_M_Inst2")
        (else
          (Rendering|Material|SetMaterial (Variables|Default|GetSkeletalMesh) 2 "/Game/MAIN/Pokemon/Cars/Mini/PokeCarBody_M_Inst3.PokeCarBody_M_Inst3"))))
    (elif (Math|Random|RandomBoolwithWeight 0.5)
      (Rendering|Material|SetMaterial (Variables|Default|GetSkeletalMesh) 2 "/Game/MAIN/Pokemon/Cars/Mini/PokeCarBody_M_Inst4.PokeCarBody_M_Inst4")
      (elif (Math|Random|RandomBoolwithWeight 0.5)
        (Rendering|Material|SetMaterial (Variables|Default|GetSkeletalMesh) 2 "/Game/MAIN/Pokemon/Cars/Mini/PokeCarBody_M_Inst5.PokeCarBody_M_Inst5")
        (else
          (Rendering|Material|SetMaterial (Variables|Default|GetSkeletalMesh) 2 "/Game/MAIN/Pokemon/Cars/Mini/PokeCarBody_M_Inst_Inst.PokeCarBody_M_Inst_Inst")))))
  (return))