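; Pokémon den actor that hosts Dynamax battles, randomly rerolling whether it is active and showing beams when it is.
; Interacting with a summoned pet saves and boosts its health, hands the player control, then teleports and enlarges it.
; Behind a loading screen, it spawns a giant hostile opponent from weighted rarity pools.
; Tick-detected opponent death or recall cleanup restores the pet's health, size, speed and camera, switches music and empties the den.
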(event Custom|SaveHealthOfPlayerPokemon
  (bind _returnvalue (Game|GetPlayerController 0))
  (Variables|/Game/MAIN/PetSystem/Pets/Parent/Pet_Parent_BP.Pet_Parent_BP_C|SetMinHealthToSaveDen (stale EventInteract _toggledpet) (.currenthealth (Variables|/Game/MAIN/PetSystem/Pets/Parent/Pet_Parent_BP.Pet_Parent_BP_C|GetPetStructure (stale EventInteract _toggledpet))))
  (Variables|/Game/MAIN/PetSystem/Pets/Parent/Pet_Parent_BP.Pet_Parent_BP_C|SetMaxHealthToSaveDen (stale EventInteract _toggledpet) (.maxhealth (Variables|/Game/MAIN/PetSystem/Pets/Parent/Pet_Parent_BP.Pet_Parent_BP_C|GetPetStructure (stale EventInteract _toggledpet))))
  (Variables|/Game/MAIN/PetSystem/Pets/Parent/Pet_Parent_BP.Pet_Parent_BP_C|SetPetStructure (stale EventInteract _toggledpet) (Utilities|Struct|MakePoStructure (.name (Variables|/Game/MAIN/PetSystem/Pets/Parent/Pet_Parent_BP.Pet_Parent_BP_C|GetPetStructure (stale EventInteract _toggledpet))) (.isstackable (Variables|/Game/MAIN/PetSystem/Pets/Parent/Pet_Parent_BP.Pet_Parent_BP_C|GetPetStructure (stale EventInteract _toggledpet))) (.thumbnail (Variables|/Game/MAIN/PetSystem/Pets/Parent/Pet_Parent_BP.Pet_Parent_BP_C|GetPetStructure (stale EventInteract _toggledpet))) (.maxstacksize (Variables|/Game/MAIN/PetSystem/Pets/Parent/Pet_Parent_BP.Pet_Parent_BP_C|GetPetStructure (stale EventInteract _toggledpet))) (.isconsumable (Variables|/Game/MAIN/PetSystem/Pets/Parent/Pet_Parent_BP.Pet_Parent_BP_C|GetPetStructure (stale EventInteract _toggledpet))) (.description (Variables|/Game/MAIN/PetSystem/Pets/Parent/Pet_Parent_BP.Pet_Parent_BP_C|GetPetStructure (stale EventInteract _toggledpet))) (.pokédexno (Variables|/Game/MAIN/PetSystem/Pets/Parent/Pet_Parent_BP.Pet_Parent_BP_C|GetPetStructure (stale EventInteract _toggledpet))) (.species (Variables|/Game/MAIN/PetSystem/Pets/Parent/Pet_Parent_BP.Pet_Parent_BP_C|GetPetStructure (stale EventInteract _toggledpet))) (.class (Variables|/Game/MAIN/PetSystem/Pets/Parent/Pet_Parent_BP.Pet_Parent_BP_C|GetPetStructure (stale EventInteract _toggledpet))) (.pettag (Variables|/Game/MAIN/PetSystem/Pets/Parent/Pet_Parent_BP.Pet_Parent_BP_C|GetPetStructure (stale EventInteract _toggledpet))) (.pettype (Variables|/Game/MAIN/PetSystem/Pets/Parent/Pet_Parent_BP.Pet_Parent_BP_C|GetPetStructure (stale EventInteract _toggledpet))) (.pettype2 (Variables|/Game/MAIN/PetSystem/Pets/Parent/Pet_Parent_BP.Pet_Parent_BP_C|GetPetStructure (stale EventInteract _toggledpet))) (.raretype (Variables|/Game/MAIN/PetSystem/Pets/Parent/Pet_Parent_BP.Pet_Parent_BP_C|GetPetStructure (stale EventInteract _toggledpet))) (.nature (Variables|/Game/MAIN/PetSystem/Pets/Parent/Pet_Parent_BP.Pet_Parent_BP_C|GetPetStructure (stale EventInteract _toggledpet))) (.ivs (Variables|/Game/MAIN/PetSystem/Pets/Parent/Pet_Parent_BP.Pet_Parent_BP_C|GetPetStructure (stale EventInteract _toggledpet))) (.evs (Variables|/Game/MAIN/PetSystem/Pets/Parent/Pet_Parent_BP.Pet_Parent_BP_C|GetPetStructure (stale EventInteract _toggledpet))) (.cannotbepickedup (Variables|/Game/MAIN/PetSystem/Pets/Parent/Pet_Parent_BP.Pet_Parent_BP_C|GetPetStructure (stale EventInteract _toggledpet))) (.trainerownedby (Variables|/Game/MAIN/PetSystem/Pets/Parent/Pet_Parent_BP.Pet_Parent_BP_C|GetPetStructure (stale EventInteract _toggledpet))) (.cost (Variables|/Game/MAIN/PetSystem/Pets/Parent/Pet_Parent_BP.Pet_Parent_BP_C|GetPetStructure (stale EventInteract _toggledpet))) (.level (Variables|/Game/MAIN/PetSystem/Pets/Parent/Pet_Parent_BP.Pet_Parent_BP_C|GetPetStructure (stale EventInteract _toggledpet))) (+ (.currenthealth (Variables|/Game/MAIN/PetSystem/Pets/Parent/Pet_Parent_BP.Pet_Parent_BP_C|GetPetStructure (stale EventInteract _toggledpet))) 200) (+ (.maxhealth (Variables|/Game/MAIN/PetSystem/Pets/Parent/Pet_Parent_BP.Pet_Parent_BP_C|GetPetStructure (stale EventInteract _toggledpet))) 200) (.mindamage (Variables|/Game/MAIN/PetSystem/Pets/Parent/Pet_Parent_BP.Pet_Parent_BP_C|GetPetStructure (stale EventInteract _toggledpet))) (.maxdamage (Variables|/Game/MAIN/PetSystem/Pets/Parent/Pet_Parent_BP.Pet_Parent_BP_C|GetPetStructure (stale EventInteract _toggledpet))) (.currentmana (Variables|/Game/MAIN/PetSystem/Pets/Parent/Pet_Parent_BP.Pet_Parent_BP_C|GetPetStructure (stale EventInteract _toggledpet))) (.maxmana (Variables|/Game/MAIN/PetSystem/Pets/Parent/Pet_Parent_BP.Pet_Parent_BP_C|GetPetStructure (stale EventInteract _toggledpet))) (.happyness (Variables|/Game/MAIN/PetSystem/Pets/Parent/Pet_Parent_BP.Pet_Parent_BP_C|GetPetStructure (stale EventInteract _toggledpet))) (.isownedbyplayer (Variables|/Game/MAIN/PetSystem/Pets/Parent/Pet_Parent_BP.Pet_Parent_BP_C|GetPetStructure (stale EventInteract _toggledpet))) (.isdead (Variables|/Game/MAIN/PetSystem/Pets/Parent/Pet_Parent_BP.Pet_Parent_BP_C|GetPetStructure (stale EventInteract _toggledpet))) (.issummoned (Variables|/Game/MAIN/PetSystem/Pets/Parent/Pet_Parent_BP.Pet_Parent_BP_C|GetPetStructure (stale EventInteract _toggledpet))) (.iswild (Variables|/Game/MAIN/PetSystem/Pets/Parent/Pet_Parent_BP.Pet_Parent_BP_C|GetPetStructure (stale EventInteract _toggledpet))) (.isattacking (Variables|/Game/MAIN/PetSystem/Pets/Parent/Pet_Parent_BP.Pet_Parent_BP_C|GetPetStructure (stale EventInteract _toggledpet))) (.isusingability1 (Variables|/Game/MAIN/PetSystem/Pets/Parent/Pet_Parent_BP.Pet_Parent_BP_C|GetPetStructure (stale EventInteract _toggledpet))) (.isusingability2 (Variables|/Game/MAIN/PetSystem/Pets/Parent/Pet_Parent_BP.Pet_Parent_BP_C|GetPetStructure (stale EventInteract _toggledpet))) (.isusingability3 (Variables|/Game/MAIN/PetSystem/Pets/Parent/Pet_Parent_BP.Pet_Parent_BP_C|GetPetStructure (stale EventInteract _toggledpet))) (.isusingability4 (Variables|/Game/MAIN/PetSystem/Pets/Parent/Pet_Parent_BP.Pet_Parent_BP_C|GetPetStructure (stale EventInteract _toggledpet))) (.isshiny (Variables|/Game/MAIN/PetSystem/Pets/Parent/Pet_Parent_BP.Pet_Parent_BP_C|GetPetStructure (stale EventInteract _toggledpet))) (.ismetallic (Variables|/Game/MAIN/PetSystem/Pets/Parent/Pet_Parent_BP.Pet_Parent_BP_C|GetPetStructure (stale EventInteract _toggledpet))) (.isghostly (Variables|/Game/MAIN/PetSystem/Pets/Parent/Pet_Parent_BP.Pet_Parent_BP_C|GetPetStructure (stale EventInteract _toggledpet))) (.petsize (Variables|/Game/MAIN/PetSystem/Pets/Parent/Pet_Parent_BP.Pet_Parent_BP_C|GetPetStructure (stale EventInteract _toggledpet))) (.issellable (Variables|/Game/MAIN/PetSystem/Pets/Parent/Pet_Parent_BP.Pet_Parent_BP_C|GetPetStructure (stale EventInteract _toggledpet))) (.canevolve (Variables|/Game/MAIN/PetSystem/Pets/Parent/Pet_Parent_BP.Pet_Parent_BP_C|GetPetStructure (stale EventInteract _toggledpet))) (.hasevolved (Variables|/Game/MAIN/PetSystem/Pets/Parent/Pet_Parent_BP.Pet_Parent_BP_C|GetPetStructure (stale EventInteract _toggledpet))) (.evolvesinto (Variables|/Game/MAIN/PetSystem/Pets/Parent/Pet_Parent_BP.Pet_Parent_BP_C|GetPetStructure (stale EventInteract _toggledpet))) (.currentxp (Variables|/Game/MAIN/PetSystem/Pets/Parent/Pet_Parent_BP.Pet_Parent_BP_C|GetPetStructure (stale EventInteract _toggledpet))) (.neededxp (Variables|/Game/MAIN/PetSystem/Pets/Parent/Pet_Parent_BP.Pet_Parent_BP_C|GetPetStructure (stale EventInteract _toggledpet)))))
  (bind _playerreference (Variables|Default|GetPlayerReference)
    (:then
      (Default|ControlPokemon _playerreference)
      (Variables|/Game/MAIN/Blueprints/Player/MasterCharacter_BP.MasterCharacter_BP_C|SetIsPetPlayerControlled _playerreference true)
      (Variables|/Script/Engine.PlayerController|SetbShowMouseCursor _returnvalue false)
      (Input|SetInputModeGameOnly _returnvalue)
      (Utilities|FlowControl|Delay 4.0)
      (CallFunction|SetPlayersPokemonforDenBattle))
    (:else)))

(event Custom|SetPlayersPokemonForDenBattle
  (Transformation|SetActorLocation (stale EventInteract _toggledpet) (Transformation|GetWorldLocation (Variables|Default|GetPlayerPokemonSpawnPoint)) false false)
  (Variables|/Script/Engine.CharacterMovementComponent|SetMaxWalkSpeed (Variables|/Script/Engine.Character|GetCharacterMovement (stale EventInteract _toggledpet)) (Variables|Default|GetMaxDynamaxWalkSpeed))
  (Utilities|FlowControl|Delay 0.5)
  (if (== (.class (Variables|/Game/MAIN/PetSystem/Pets/Parent/Pet_Parent_BP.Pet_Parent_BP_C|GetPetStructure (stale EventInteract _toggledpet))) "/Game/MAIN/PetSystem/Pets/Pokemon/Golbat_BP.Golbat_BP_C")
    (Transformation|SetActorScale3D (stale EventInteract _toggledpet) "40.000000,40.000000,40.000000")
    (else
      (Transformation|SetActorScale3D (stale EventInteract _toggledpet) (Variables|Default|GetDynamaxScale))))
  (CallFunction|SetPlayerPokemonScales))

(event Custom|ControlPokemonInDen
  (CallFunction|SpawnDenPokemon)
  (Utilities|FlowControl|Delay 6e+01)
  (bind _asrpg_game_mode (Utilities|Casting|CastToRPG_GameMode (Game|GetGameMode)))
  (Default|PlayDenBattleMusic _asrpg_game_mode)
  (Utilities|FlowControl|Delay 8.0)
  (bind _loadingui (Variables|Default|GetLoadingUI)
    (:then
      (Widget|RemovefromParent _loadingui))
    (:else
      _))
  (Variables|Default|SetLoadingUI 0)
  (Audio|PlaySound2D "/Game/MAIN/Pokemon/Sound/DynamaxRoar_Cue.DynamaxRoar_Cue" 1.0 1.0 0.0 0 0))

(event Custom|ResetPlayerPokemonHealthToNormal
  (bind _playerreference (Variables|Default|GetPlayerReference)
    (:then
      (bind _toggledpet (Variables|/Game/MAIN/Blueprints/Player/MasterCharacter_BP.MasterCharacter_BP_C|GetToggledPet _playerreference)
        (:then
          (Variables|/Game/MAIN/PetSystem/Pets/Parent/Pet_Parent_BP.Pet_Parent_BP_C|SetPetStructure _toggledpet (Utilities|Struct|MakePoStructure (.name (Variables|/Game/MAIN/PetSystem/Pets/Parent/Pet_Parent_BP.Pet_Parent_BP_C|GetPetStructure _toggledpet)) (.isstackable (Variables|/Game/MAIN/PetSystem/Pets/Parent/Pet_Parent_BP.Pet_Parent_BP_C|GetPetStructure _toggledpet)) (.thumbnail (Variables|/Game/MAIN/PetSystem/Pets/Parent/Pet_Parent_BP.Pet_Parent_BP_C|GetPetStructure _toggledpet)) (.maxstacksize (Variables|/Game/MAIN/PetSystem/Pets/Parent/Pet_Parent_BP.Pet_Parent_BP_C|GetPetStructure _toggledpet)) (.isconsumable (Variables|/Game/MAIN/PetSystem/Pets/Parent/Pet_Parent_BP.Pet_Parent_BP_C|GetPetStructure _toggledpet)) (.description (Variables|/Game/MAIN/PetSystem/Pets/Parent/Pet_Parent_BP.Pet_Parent_BP_C|GetPetStructure _toggledpet)) (.pokédexno (Variables|/Game/MAIN/PetSystem/Pets/Parent/Pet_Parent_BP.Pet_Parent_BP_C|GetPetStructure _toggledpet)) (.species (Variables|/Game/MAIN/PetSystem/Pets/Parent/Pet_Parent_BP.Pet_Parent_BP_C|GetPetStructure _toggledpet)) (.class (Variables|/Game/MAIN/PetSystem/Pets/Parent/Pet_Parent_BP.Pet_Parent_BP_C|GetPetStructure _toggledpet)) (.pettag (Variables|/Game/MAIN/PetSystem/Pets/Parent/Pet_Parent_BP.Pet_Parent_BP_C|GetPetStructure _toggledpet)) (.pettype (Variables|/Game/MAIN/PetSystem/Pets/Parent/Pet_Parent_BP.Pet_Parent_BP_C|GetPetStructure _toggledpet)) (.pettype2 (Variables|/Game/MAIN/PetSystem/Pets/Parent/Pet_Parent_BP.Pet_Parent_BP_C|GetPetStructure _toggledpet)) (.raretype (Variables|/Game/MAIN/PetSystem/Pets/Parent/Pet_Parent_BP.Pet_Parent_BP_C|GetPetStructure _toggledpet)) (.nature (Variables|/Game/MAIN/PetSystem/Pets/Parent/Pet_Parent_BP.Pet_Parent_BP_C|GetPetStructure _toggledpet)) (.ivs (Variables|/Game/MAIN/PetSystem/Pets/Parent/Pet_Parent_BP.Pet_Parent_BP_C|GetPetStructure _toggledpet)) (.evs (Variables|/Game/MAIN/PetSystem/Pets/Parent/Pet_Parent_BP.Pet_Parent_BP_C|GetPetStructure _toggledpet)) (.cannotbepickedup (Variables|/Game/MAIN/PetSystem/Pets/Parent/Pet_Parent_BP.Pet_Parent_BP_C|GetPetStructure _toggledpet)) (.trainerownedby (Variables|/Game/MAIN/PetSystem/Pets/Parent/Pet_Parent_BP.Pet_Parent_BP_C|GetPetStructure _toggledpet)) (.cost (Variables|/Game/MAIN/PetSystem/Pets/Parent/Pet_Parent_BP.Pet_Parent_BP_C|GetPetStructure _toggledpet)) (.level (Variables|/Game/MAIN/PetSystem/Pets/Parent/Pet_Parent_BP.Pet_Parent_BP_C|GetPetStructure _toggledpet)) (Variables|/Game/MAIN/PetSystem/Pets/Parent/Pet_Parent_BP.Pet_Parent_BP_C|GetMinHealthToSaveDen _toggledpet) (Variables|/Game/MAIN/PetSystem/Pets/Parent/Pet_Parent_BP.Pet_Parent_BP_C|GetMaxHealthToSaveDen _toggledpet) (.mindamage (Variables|/Game/MAIN/PetSystem/Pets/Parent/Pet_Parent_BP.Pet_Parent_BP_C|GetPetStructure _toggledpet)) (.maxdamage (Variables|/Game/MAIN/PetSystem/Pets/Parent/Pet_Parent_BP.Pet_Parent_BP_C|GetPetStructure _toggledpet)) (.currentmana (Variables|/Game/MAIN/PetSystem/Pets/Parent/Pet_Parent_BP.Pet_Parent_BP_C|GetPetStructure _toggledpet)) (.maxmana (Variables|/Game/MAIN/PetSystem/Pets/Parent/Pet_Parent_BP.Pet_Parent_BP_C|GetPetStructure _toggledpet)) (.happyness (Variables|/Game/MAIN/PetSystem/Pets/Parent/Pet_Parent_BP.Pet_Parent_BP_C|GetPetStructure _toggledpet)) (.isownedbyplayer (Variables|/Game/MAIN/PetSystem/Pets/Parent/Pet_Parent_BP.Pet_Parent_BP_C|GetPetStructure _toggledpet)) (.isdead (Variables|/Game/MAIN/PetSystem/Pets/Parent/Pet_Parent_BP.Pet_Parent_BP_C|GetPetStructure _toggledpet)) (.issummoned (Variables|/Game/MAIN/PetSystem/Pets/Parent/Pet_Parent_BP.Pet_Parent_BP_C|GetPetStructure _toggledpet)) (.iswild (Variables|/Game/MAIN/PetSystem/Pets/Parent/Pet_Parent_BP.Pet_Parent_BP_C|GetPetStructure _toggledpet)) (.isattacking (Variables|/Game/MAIN/PetSystem/Pets/Parent/Pet_Parent_BP.Pet_Parent_BP_C|GetPetStructure _toggledpet)) (.isusingability1 (Variables|/Game/MAIN/PetSystem/Pets/Parent/Pet_Parent_BP.Pet_Parent_BP_C|GetPetStructure _toggledpet)) (.isusingability2 (Variables|/Game/MAIN/PetSystem/Pets/Parent/Pet_Parent_BP.Pet_Parent_BP_C|GetPetStructure _toggledpet)) (.isusingability3 (Variables|/Game/MAIN/PetSystem/Pets/Parent/Pet_Parent_BP.Pet_Parent_BP_C|GetPetStructure _toggledpet)) (.isusingability4 (Variables|/Game/MAIN/PetSystem/Pets/Parent/Pet_Parent_BP.Pet_Parent_BP_C|GetPetStructure _toggledpet)) (.isshiny (Variables|/Game/MAIN/PetSystem/Pets/Parent/Pet_Parent_BP.Pet_Parent_BP_C|GetPetStructure _toggledpet)) (.ismetallic (Variables|/Game/MAIN/PetSystem/Pets/Parent/Pet_Parent_BP.Pet_Parent_BP_C|GetPetStructure _toggledpet)) (.isghostly (Variables|/Game/MAIN/PetSystem/Pets/Parent/Pet_Parent_BP.Pet_Parent_BP_C|GetPetStructure _toggledpet)) (.petsize (Variables|/Game/MAIN/PetSystem/Pets/Parent/Pet_Parent_BP.Pet_Parent_BP_C|GetPetStructure _toggledpet)) (.issellable (Variables|/Game/MAIN/PetSystem/Pets/Parent/Pet_Parent_BP.Pet_Parent_BP_C|GetPetStructure _toggledpet)) (.canevolve (Variables|/Game/MAIN/PetSystem/Pets/Parent/Pet_Parent_BP.Pet_Parent_BP_C|GetPetStructure _toggledpet)) (.hasevolved (Variables|/Game/MAIN/PetSystem/Pets/Parent/Pet_Parent_BP.Pet_Parent_BP_C|GetPetStructure _toggledpet)) (.evolvesinto (Variables|/Game/MAIN/PetSystem/Pets/Parent/Pet_Parent_BP.Pet_Parent_BP_C|GetPetStructure _toggledpet)) (.currentxp (Variables|/Game/MAIN/PetSystem/Pets/Parent/Pet_Parent_BP.Pet_Parent_BP_C|GetPetStructure _toggledpet)) (.neededxp (Variables|/Game/MAIN/PetSystem/Pets/Parent/Pet_Parent_BP.Pet_Parent_BP_C|GetPetStructure _toggledpet))))
          (Variables|/Script/Engine.SpringArmComponent|SetTargetArmLength (Variables|/Game/MAIN/PetSystem/Pets/Parent/Pet_Parent_BP.Pet_Parent_BP_C|GetCameraBoom _toggledpet) 4e+02)
          (Variables|/Game/MAIN/PetSystem/Pets/Parent/Pet_Parent_BP.Pet_Parent_BP_C|SetZoomInteval _toggledpet 5e+01))
        (:else)))
    (:else)))

(event Custom|SpawnDenPokemon
  (if (Math|Random|RandomBoolwithWeight (Variables|Default|GetCommonSpawnRate))
    (Variables|Default|GetSpawnedPokemon
      (:then)
      (:else
        (bind _returnvalue (AI|SpawnAIFromClass (Utilities|Array|Get(acopy) (Variables|Default|GetCommonSpawns) (Math|Random|RandomIntegerinRange 0 7)) 0 (Transformation|GetWorldLocation (Variables|Default|GetWildSpawnPoint)) "0, 0, 0" true))
        (bind _output_get (Variables|Default|SetSpawnedPokemon _returnvalue))
        (bind _aspet_parent_bp (Utilities|Casting|CastToPet_Parent_BP _output_get))
        (bind _output_get_2 (Variables|Default|SetSpawnedDynamaxPokemon _aspet_parent_bp))
        (Transformation|SetActorScale3D _output_get_2 (Variables|Default|GetDynamaxScale))
        (Variables|/Script/Engine.CharacterMovementComponent|SetMaxWalkSpeed (Variables|/Script/Engine.Character|GetCharacterMovement _output_get_2) (Variables|Default|GetMaxDynamaxWalkSpeed))
        (Variables|/Game/MAIN/PetSystem/Pets/Parent/Pet_Parent_BP.Pet_Parent_BP_C|SetPetStructure _output_get_2 (Utilities|Struct|MakePoStructure (.name (Variables|/Game/MAIN/PetSystem/Pets/Parent/Pet_Parent_BP.Pet_Parent_BP_C|GetPetStructure _output_get_2)) (.isstackable (Variables|/Game/MAIN/PetSystem/Pets/Parent/Pet_Parent_BP.Pet_Parent_BP_C|GetPetStructure _output_get_2)) (.thumbnail (Variables|/Game/MAIN/PetSystem/Pets/Parent/Pet_Parent_BP.Pet_Parent_BP_C|GetPetStructure _output_get_2)) (.maxstacksize (Variables|/Game/MAIN/PetSystem/Pets/Parent/Pet_Parent_BP.Pet_Parent_BP_C|GetPetStructure _output_get_2)) (.isconsumable (Variables|/Game/MAIN/PetSystem/Pets/Parent/Pet_Parent_BP.Pet_Parent_BP_C|GetPetStructure _output_get_2)) (.description (Variables|/Game/MAIN/PetSystem/Pets/Parent/Pet_Parent_BP.Pet_Parent_BP_C|GetPetStructure _output_get_2)) (.pokédexno (Variables|/Game/MAIN/PetSystem/Pets/Parent/Pet_Parent_BP.Pet_Parent_BP_C|GetPetStructure _output_get_2)) (.species (Variables|/Game/MAIN/PetSystem/Pets/Parent/Pet_Parent_BP.Pet_Parent_BP_C|GetPetStructure _output_get_2)) (.class (Variables|/Game/MAIN/PetSystem/Pets/Parent/Pet_Parent_BP.Pet_Parent_BP_C|GetPetStructure _output_get_2)) (.pettag (Variables|/Game/MAIN/PetSystem/Pets/Parent/Pet_Parent_BP.Pet_Parent_BP_C|GetPetStructure _output_get_2)) (.pettype (Variables|/Game/MAIN/PetSystem/Pets/Parent/Pet_Parent_BP.Pet_Parent_BP_C|GetPetStructure _output_get_2)) (.pettype2 (Variables|/Game/MAIN/PetSystem/Pets/Parent/Pet_Parent_BP.Pet_Parent_BP_C|GetPetStructure _output_get_2)) (.raretype (Variables|/Game/MAIN/PetSystem/Pets/Parent/Pet_Parent_BP.Pet_Parent_BP_C|GetPetStructure _output_get_2)) (.nature (Variables|/Game/MAIN/PetSystem/Pets/Parent/Pet_Parent_BP.Pet_Parent_BP_C|GetPetStructure _output_get_2)) (.ivs (Variables|/Game/MAIN/PetSystem/Pets/Parent/Pet_Parent_BP.Pet_Parent_BP_C|GetPetStructure _output_get_2)) (.evs (Variables|/Game/MAIN/PetSystem/Pets/Parent/Pet_Parent_BP.Pet_Parent_BP_C|GetPetStructure _output_get_2)) (.cannotbepickedup (Variables|/Game/MAIN/PetSystem/Pets/Parent/Pet_Parent_BP.Pet_Parent_BP_C|GetPetStructure _output_get_2)) (.trainerownedby (Variables|/Game/MAIN/PetSystem/Pets/Parent/Pet_Parent_BP.Pet_Parent_BP_C|GetPetStructure _output_get_2)) (.cost (Variables|/Game/MAIN/PetSystem/Pets/Parent/Pet_Parent_BP.Pet_Parent_BP_C|GetPetStructure _output_get_2)) (.level (Variables|/Game/MAIN/PetSystem/Pets/Parent/Pet_Parent_BP.Pet_Parent_BP_C|GetPetStructure _output_get_2)) (+ (.currenthealth (Variables|/Game/MAIN/PetSystem/Pets/Parent/Pet_Parent_BP.Pet_Parent_BP_C|GetPetStructure _output_get_2)) 100) (+ (.maxhealth (Variables|/Game/MAIN/PetSystem/Pets/Parent/Pet_Parent_BP.Pet_Parent_BP_C|GetPetStructure _output_get_2)) 100) (.mindamage (Variables|/Game/MAIN/PetSystem/Pets/Parent/Pet_Parent_BP.Pet_Parent_BP_C|GetPetStructure _output_get_2)) (.maxdamage (Variables|/Game/MAIN/PetSystem/Pets/Parent/Pet_Parent_BP.Pet_Parent_BP_C|GetPetStructure _output_get_2)) (.currentmana (Variables|/Game/MAIN/PetSystem/Pets/Parent/Pet_Parent_BP.Pet_Parent_BP_C|GetPetStructure _output_get_2)) (.maxmana (Variables|/Game/MAIN/PetSystem/Pets/Parent/Pet_Parent_BP.Pet_Parent_BP_C|GetPetStructure _output_get_2)) (.happyness (Variables|/Game/MAIN/PetSystem/Pets/Parent/Pet_Parent_BP.Pet_Parent_BP_C|GetPetStructure _output_get_2)) false (.isdead (Variables|/Game/MAIN/PetSystem/Pets/Parent/Pet_Parent_BP.Pet_Parent_BP_C|GetPetStructure _output_get_2)) (.issummoned (Variables|/Game/MAIN/PetSystem/Pets/Parent/Pet_Parent_BP.Pet_Parent_BP_C|GetPetStructure _output_get_2)) true (.isattacking (Variables|/Game/MAIN/PetSystem/Pets/Parent/Pet_Parent_BP.Pet_Parent_BP_C|GetPetStructure _output_get_2)) (.isusingability1 (Variables|/Game/MAIN/PetSystem/Pets/Parent/Pet_Parent_BP.Pet_Parent_BP_C|GetPetStructure _output_get_2)) (.isusingability2 (Variables|/Game/MAIN/PetSystem/Pets/Parent/Pet_Parent_BP.Pet_Parent_BP_C|GetPetStructure _output_get_2)) (.isusingability3 (Variables|/Game/MAIN/PetSystem/Pets/Parent/Pet_Parent_BP.Pet_Parent_BP_C|GetPetStructure _output_get_2)) (.isusingability4 (Variables|/Game/MAIN/PetSystem/Pets/Parent/Pet_Parent_BP.Pet_Parent_BP_C|GetPetStructure _output_get_2)) (.isshiny (Variables|/Game/MAIN/PetSystem/Pets/Parent/Pet_Parent_BP.Pet_Parent_BP_C|GetPetStructure _output_get_2)) (.ismetallic (Variables|/Game/MAIN/PetSystem/Pets/Parent/Pet_Parent_BP.Pet_Parent_BP_C|GetPetStructure _output_get_2)) (.isghostly (Variables|/Game/MAIN/PetSystem/Pets/Parent/Pet_Parent_BP.Pet_Parent_BP_C|GetPetStructure _output_get_2)) (.petsize (Variables|/Game/MAIN/PetSystem/Pets/Parent/Pet_Parent_BP.Pet_Parent_BP_C|GetPetStructure _output_get_2)) (.issellable (Variables|/Game/MAIN/PetSystem/Pets/Parent/Pet_Parent_BP.Pet_Parent_BP_C|GetPetStructure _output_get_2)) (.canevolve (Variables|/Game/MAIN/PetSystem/Pets/Parent/Pet_Parent_BP.Pet_Parent_BP_C|GetPetStructure _output_get_2)) (.hasevolved (Variables|/Game/MAIN/PetSystem/Pets/Parent/Pet_Parent_BP.Pet_Parent_BP_C|GetPetStructure _output_get_2)) (.evolvesinto (Variables|/Game/MAIN/PetSystem/Pets/Parent/Pet_Parent_BP.Pet_Parent_BP_C|GetPetStructure _output_get_2)) (.currentxp (Variables|/Game/MAIN/PetSystem/Pets/Parent/Pet_Parent_BP.Pet_Parent_BP_C|GetPetStructure _output_get_2)) (.neededxp (Variables|/Game/MAIN/PetSystem/Pets/Parent/Pet_Parent_BP.Pet_Parent_BP_C|GetPetStructure _output_get_2))))
        (Variables|/Game/MAIN/PetSystem/Pets/Parent/Pet_Parent_BP.Pet_Parent_BP_C|SetIsHostile _output_get_2 true)
        (CallFunction|SetEnemyScales)))
    (elif (Math|Random|RandomBoolwithWeight (Variables|Default|GetUncommonSpawnRate))
      (Variables|Default|GetSpawnedPokemon
        (:then)
        (:else
          (bind _returnvalue_2 (AI|SpawnAIFromClass (Utilities|Array|Get(acopy) (Variables|Default|GetUncommonSpawns) (Math|Random|RandomIntegerinRange 0 3)) 0 (Transformation|GetWorldLocation (Variables|Default|GetWildSpawnPoint)) "0, 0, 0" true))
          (bind _output_get_3 (Variables|Default|SetSpawnedPokemon _returnvalue_2))
          (bind _aspet_parent_bp_2 (Utilities|Casting|CastToPet_Parent_BP _output_get_3))
          (bind _output_get_4 (Variables|Default|SetSpawnedDynamaxPokemon _aspet_parent_bp_2))
          (Transformation|SetActorScale3D _output_get_4 (Variables|Default|GetDynamaxScale))
          (Variables|/Script/Engine.CharacterMovementComponent|SetMaxWalkSpeed (Variables|/Script/Engine.Character|GetCharacterMovement _output_get_4) (Variables|Default|GetMaxDynamaxWalkSpeed))
          (Variables|/Game/MAIN/PetSystem/Pets/Parent/Pet_Parent_BP.Pet_Parent_BP_C|SetPetStructure _output_get_4 (Utilities|Struct|MakePoStructure (.name (Variables|/Game/MAIN/PetSystem/Pets/Parent/Pet_Parent_BP.Pet_Parent_BP_C|GetPetStructure _output_get_4)) (.isstackable (Variables|/Game/MAIN/PetSystem/Pets/Parent/Pet_Parent_BP.Pet_Parent_BP_C|GetPetStructure _output_get_4)) (.thumbnail (Variables|/Game/MAIN/PetSystem/Pets/Parent/Pet_Parent_BP.Pet_Parent_BP_C|GetPetStructure _output_get_4)) (.maxstacksize (Variables|/Game/MAIN/PetSystem/Pets/Parent/Pet_Parent_BP.Pet_Parent_BP_C|GetPetStructure _output_get_4)) (.isconsumable (Variables|/Game/MAIN/PetSystem/Pets/Parent/Pet_Parent_BP.Pet_Parent_BP_C|GetPetStructure _output_get_4)) (.description (Variables|/Game/MAIN/PetSystem/Pets/Parent/Pet_Parent_BP.Pet_Parent_BP_C|GetPetStructure _output_get_4)) (.pokédexno (Variables|/Game/MAIN/PetSystem/Pets/Parent/Pet_Parent_BP.Pet_Parent_BP_C|GetPetStructure _output_get_4)) (.species (Variables|/Game/MAIN/PetSystem/Pets/Parent/Pet_Parent_BP.Pet_Parent_BP_C|GetPetStructure _output_get_4)) (.class (Variables|/Game/MAIN/PetSystem/Pets/Parent/Pet_Parent_BP.Pet_Parent_BP_C|GetPetStructure _output_get_4)) (.pettag (Variables|/Game/MAIN/PetSystem/Pets/Parent/Pet_Parent_BP.Pet_Parent_BP_C|GetPetStructure _output_get_4)) (.pettype (Variables|/Game/MAIN/PetSystem/Pets/Parent/Pet_Parent_BP.Pet_Parent_BP_C|GetPetStructure _output_get_4)) (.pettype2 (Variables|/Game/MAIN/PetSystem/Pets/Parent/Pet_Parent_BP.Pet_Parent_BP_C|GetPetStructure _output_get_4)) (.raretype (Variables|/Game/MAIN/PetSystem/Pets/Parent/Pet_Parent_BP.Pet_Parent_BP_C|GetPetStructure _output_get_4)) (.nature (Variables|/Game/MAIN/PetSystem/Pets/Parent/Pet_Parent_BP.Pet_Parent_BP_C|GetPetStructure _output_get_4)) (.ivs (Variables|/Game/MAIN/PetSystem/Pets/Parent/Pet_Parent_BP.Pet_Parent_BP_C|GetPetStructure _output_get_4)) (.evs (Variables|/Game/MAIN/PetSystem/Pets/Parent/Pet_Parent_BP.Pet_Parent_BP_C|GetPetStructure _output_get_4)) (.cannotbepickedup (Variables|/Game/MAIN/PetSystem/Pets/Parent/Pet_Parent_BP.Pet_Parent_BP_C|GetPetStructure _output_get_4)) (.trainerownedby (Variables|/Game/MAIN/PetSystem/Pets/Parent/Pet_Parent_BP.Pet_Parent_BP_C|GetPetStructure _output_get_4)) (.cost (Variables|/Game/MAIN/PetSystem/Pets/Parent/Pet_Parent_BP.Pet_Parent_BP_C|GetPetStructure _output_get_4)) (.level (Variables|/Game/MAIN/PetSystem/Pets/Parent/Pet_Parent_BP.Pet_Parent_BP_C|GetPetStructure _output_get_4)) (+ (.currenthealth (Variables|/Game/MAIN/PetSystem/Pets/Parent/Pet_Parent_BP.Pet_Parent_BP_C|GetPetStructure _output_get_4)) 100) (+ (.maxhealth (Variables|/Game/MAIN/PetSystem/Pets/Parent/Pet_Parent_BP.Pet_Parent_BP_C|GetPetStructure _output_get_4)) 100) (.mindamage (Variables|/Game/MAIN/PetSystem/Pets/Parent/Pet_Parent_BP.Pet_Parent_BP_C|GetPetStructure _output_get_4)) (.maxdamage (Variables|/Game/MAIN/PetSystem/Pets/Parent/Pet_Parent_BP.Pet_Parent_BP_C|GetPetStructure _output_get_4)) (.currentmana (Variables|/Game/MAIN/PetSystem/Pets/Parent/Pet_Parent_BP.Pet_Parent_BP_C|GetPetStructure _output_get_4)) (.maxmana (Variables|/Game/MAIN/PetSystem/Pets/Parent/Pet_Parent_BP.Pet_Parent_BP_C|GetPetStructure _output_get_4)) (.happyness (Variables|/Game/MAIN/PetSystem/Pets/Parent/Pet_Parent_BP.Pet_Parent_BP_C|GetPetStructure _output_get_4)) false (.isdead (Variables|/Game/MAIN/PetSystem/Pets/Parent/Pet_Parent_BP.Pet_Parent_BP_C|GetPetStructure _output_get_4)) (.issummoned (Variables|/Game/MAIN/PetSystem/Pets/Parent/Pet_Parent_BP.Pet_Parent_BP_C|GetPetStructure _output_get_4)) true (.isattacking (Variables|/Game/MAIN/PetSystem/Pets/Parent/Pet_Parent_BP.Pet_Parent_BP_C|GetPetStructure _output_get_4)) (.isusingability1 (Variables|/Game/MAIN/PetSystem/Pets/Parent/Pet_Parent_BP.Pet_Parent_BP_C|GetPetStructure _output_get_4)) (.isusingability2 (Variables|/Game/MAIN/PetSystem/Pets/Parent/Pet_Parent_BP.Pet_Parent_BP_C|GetPetStructure _output_get_4)) (.isusingability3 (Variables|/Game/MAIN/PetSystem/Pets/Parent/Pet_Parent_BP.Pet_Parent_BP_C|GetPetStructure _output_get_4)) (.isusingability4 (Variables|/Game/MAIN/PetSystem/Pets/Parent/Pet_Parent_BP.Pet_Parent_BP_C|GetPetStructure _output_get_4)) (.isshiny (Variables|/Game/MAIN/PetSystem/Pets/Parent/Pet_Parent_BP.Pet_Parent_BP_C|GetPetStructure _output_get_4)) (.ismetallic (Variables|/Game/MAIN/PetSystem/Pets/Parent/Pet_Parent_BP.Pet_Parent_BP_C|GetPetStructure _output_get_4)) (.isghostly (Variables|/Game/MAIN/PetSystem/Pets/Parent/Pet_Parent_BP.Pet_Parent_BP_C|GetPetStructure _output_get_4)) (.petsize (Variables|/Game/MAIN/PetSystem/Pets/Parent/Pet_Parent_BP.Pet_Parent_BP_C|GetPetStructure _output_get_4)) (.issellable (Variables|/Game/MAIN/PetSystem/Pets/Parent/Pet_Parent_BP.Pet_Parent_BP_C|GetPetStructure _output_get_4)) (.canevolve (Variables|/Game/MAIN/PetSystem/Pets/Parent/Pet_Parent_BP.Pet_Parent_BP_C|GetPetStructure _output_get_4)) (.hasevolved (Variables|/Game/MAIN/PetSystem/Pets/Parent/Pet_Parent_BP.Pet_Parent_BP_C|GetPetStructure _output_get_4)) (.evolvesinto (Variables|/Game/MAIN/PetSystem/Pets/Parent/Pet_Parent_BP.Pet_Parent_BP_C|GetPetStructure _output_get_4)) (.currentxp (Variables|/Game/MAIN/PetSystem/Pets/Parent/Pet_Parent_BP.Pet_Parent_BP_C|GetPetStructure _output_get_4)) (.neededxp (Variables|/Game/MAIN/PetSystem/Pets/Parent/Pet_Parent_BP.Pet_Parent_BP_C|GetPetStructure _output_get_4))))
          (Variables|/Game/MAIN/PetSystem/Pets/Parent/Pet_Parent_BP.Pet_Parent_BP_C|SetIsHostile _output_get_4 true)
          (CallFunction|SetEnemyScales)))
      (elif (Math|Random|RandomBoolwithWeight (Variables|Default|GetShinyAndMetallicCommonSpawnRate))
        (Variables|Default|GetSpawnedPokemon
          (:then)
          (:else
            (bind _returnvalue_3 (AI|SpawnAIFromClass (Utilities|Array|Get(acopy) (Variables|Default|GetShinyandMetallicCommonSpawns) (Math|Random|RandomIntegerinRange 0 9)) 0 (Transformation|GetWorldLocation (Variables|Default|GetWildSpawnPoint)) "0, 0, 0" true))
            (bind _output_get_5 (Variables|Default|SetSpawnedPokemon _returnvalue_3))
            (bind _aspet_parent_bp_3 (Utilities|Casting|CastToPet_Parent_BP _output_get_5))
            (bind _output_get_6 (Variables|Default|SetSpawnedDynamaxPokemon _aspet_parent_bp_3))
            (Transformation|SetActorScale3D _output_get_6 (Variables|Default|GetDynamaxScale))
            (Variables|/Script/Engine.CharacterMovementComponent|SetMaxWalkSpeed (Variables|/Script/Engine.Character|GetCharacterMovement _output_get_6) (Variables|Default|GetMaxDynamaxWalkSpeed))
            (Variables|/Game/MAIN/PetSystem/Pets/Parent/Pet_Parent_BP.Pet_Parent_BP_C|SetPetStructure _output_get_6 (Utilities|Struct|MakePoStructure (.name (Variables|/Game/MAIN/PetSystem/Pets/Parent/Pet_Parent_BP.Pet_Parent_BP_C|GetPetStructure _output_get_6)) (.isstackable (Variables|/Game/MAIN/PetSystem/Pets/Parent/Pet_Parent_BP.Pet_Parent_BP_C|GetPetStructure _output_get_6)) (.thumbnail (Variables|/Game/MAIN/PetSystem/Pets/Parent/Pet_Parent_BP.Pet_Parent_BP_C|GetPetStructure _output_get_6)) (.maxstacksize (Variables|/Game/MAIN/PetSystem/Pets/Parent/Pet_Parent_BP.Pet_Parent_BP_C|GetPetStructure _output_get_6)) (.isconsumable (Variables|/Game/MAIN/PetSystem/Pets/Parent/Pet_Parent_BP.Pet_Parent_BP_C|GetPetStructure _output_get_6)) (.description (Variables|/Game/MAIN/PetSystem/Pets/Parent/Pet_Parent_BP.Pet_Parent_BP_C|GetPetStructure _output_get_6)) (.pokédexno (Variables|/Game/MAIN/PetSystem/Pets/Parent/Pet_Parent_BP.Pet_Parent_BP_C|GetPetStructure _output_get_6)) (.species (Variables|/Game/MAIN/PetSystem/Pets/Parent/Pet_Parent_BP.Pet_Parent_BP_C|GetPetStructure _output_get_6)) (.class (Variables|/Game/MAIN/PetSystem/Pets/Parent/Pet_Parent_BP.Pet_Parent_BP_C|GetPetStructure _output_get_6)) (.pettag (Variables|/Game/MAIN/PetSystem/Pets/Parent/Pet_Parent_BP.Pet_Parent_BP_C|GetPetStructure _output_get_6)) (.pettype (Variables|/Game/MAIN/PetSystem/Pets/Parent/Pet_Parent_BP.Pet_Parent_BP_C|GetPetStructure _output_get_6)) (.pettype2 (Variables|/Game/MAIN/PetSystem/Pets/Parent/Pet_Parent_BP.Pet_Parent_BP_C|GetPetStructure _output_get_6)) (.raretype (Variables|/Game/MAIN/PetSystem/Pets/Parent/Pet_Parent_BP.Pet_Parent_BP_C|GetPetStructure _output_get_6)) (.nature (Variables|/Game/MAIN/PetSystem/Pets/Parent/Pet_Parent_BP.Pet_Parent_BP_C|GetPetStructure _output_get_6)) (.ivs (Variables|/Game/MAIN/PetSystem/Pets/Parent/Pet_Parent_BP.Pet_Parent_BP_C|GetPetStructure _output_get_6)) (.evs (Variables|/Game/MAIN/PetSystem/Pets/Parent/Pet_Parent_BP.Pet_Parent_BP_C|GetPetStructure _output_get_6)) (.cannotbepickedup (Variables|/Game/MAIN/PetSystem/Pets/Parent/Pet_Parent_BP.Pet_Parent_BP_C|GetPetStructure _output_get_6)) (.trainerownedby (Variables|/Game/MAIN/PetSystem/Pets/Parent/Pet_Parent_BP.Pet_Parent_BP_C|GetPetStructure _output_get_6)) (.cost (Variables|/Game/MAIN/PetSystem/Pets/Parent/Pet_Parent_BP.Pet_Parent_BP_C|GetPetStructure _output_get_6)) (.level (Variables|/Game/MAIN/PetSystem/Pets/Parent/Pet_Parent_BP.Pet_Parent_BP_C|GetPetStructure _output_get_6)) (+ (.currenthealth (Variables|/Game/MAIN/PetSystem/Pets/Parent/Pet_Parent_BP.Pet_Parent_BP_C|GetPetStructure _output_get_6)) 100) (+ (.maxhealth (Variables|/Game/MAIN/PetSystem/Pets/Parent/Pet_Parent_BP.Pet_Parent_BP_C|GetPetStructure _output_get_6)) 100) (.mindamage (Variables|/Game/MAIN/PetSystem/Pets/Parent/Pet_Parent_BP.Pet_Parent_BP_C|GetPetStructure _output_get_6)) (.maxdamage (Variables|/Game/MAIN/PetSystem/Pets/Parent/Pet_Parent_BP.Pet_Parent_BP_C|GetPetStructure _output_get_6)) (.currentmana (Variables|/Game/MAIN/PetSystem/Pets/Parent/Pet_Parent_BP.Pet_Parent_BP_C|GetPetStructure _output_get_6)) (.maxmana (Variables|/Game/MAIN/PetSystem/Pets/Parent/Pet_Parent_BP.Pet_Parent_BP_C|GetPetStructure _output_get_6)) (.happyness (Variables|/Game/MAIN/PetSystem/Pets/Parent/Pet_Parent_BP.Pet_Parent_BP_C|GetPetStructure _output_get_6)) false (.isdead (Variables|/Game/MAIN/PetSystem/Pets/Parent/Pet_Parent_BP.Pet_Parent_BP_C|GetPetStructure _output_get_6)) (.issummoned (Variables|/Game/MAIN/PetSystem/Pets/Parent/Pet_Parent_BP.Pet_Parent_BP_C|GetPetStructure _output_get_6)) true (.isattacking (Variables|/Game/MAIN/PetSystem/Pets/Parent/Pet_Parent_BP.Pet_Parent_BP_C|GetPetStructure _output_get_6)) (.isusingability1 (Variables|/Game/MAIN/PetSystem/Pets/Parent/Pet_Parent_BP.Pet_Parent_BP_C|GetPetStructure _output_get_6)) (.isusingability2 (Variables|/Game/MAIN/PetSystem/Pets/Parent/Pet_Parent_BP.Pet_Parent_BP_C|GetPetStructure _output_get_6)) (.isusingability3 (Variables|/Game/MAIN/PetSystem/Pets/Parent/Pet_Parent_BP.Pet_Parent_BP_C|GetPetStructure _output_get_6)) (.isusingability4 (Variables|/Game/MAIN/PetSystem/Pets/Parent/Pet_Parent_BP.Pet_Parent_BP_C|GetPetStructure _output_get_6)) (.isshiny (Variables|/Game/MAIN/PetSystem/Pets/Parent/Pet_Parent_BP.Pet_Parent_BP_C|GetPetStructure _output_get_6)) (.ismetallic (Variables|/Game/MAIN/PetSystem/Pets/Parent/Pet_Parent_BP.Pet_Parent_BP_C|GetPetStructure _output_get_6)) (.isghostly (Variables|/Game/MAIN/PetSystem/Pets/Parent/Pet_Parent_BP.Pet_Parent_BP_C|GetPetStructure _output_get_6)) (.petsize (Variables|/Game/MAIN/PetSystem/Pets/Parent/Pet_Parent_BP.Pet_Parent_BP_C|GetPetStructure _output_get_6)) (.issellable (Variables|/Game/MAIN/PetSystem/Pets/Parent/Pet_Parent_BP.Pet_Parent_BP_C|GetPetStructure _output_get_6)) (.canevolve (Variables|/Game/MAIN/PetSystem/Pets/Parent/Pet_Parent_BP.Pet_Parent_BP_C|GetPetStructure _output_get_6)) (.hasevolved (Variables|/Game/MAIN/PetSystem/Pets/Parent/Pet_Parent_BP.Pet_Parent_BP_C|GetPetStructure _output_get_6)) (.evolvesinto (Variables|/Game/MAIN/PetSystem/Pets/Parent/Pet_Parent_BP.Pet_Parent_BP_C|GetPetStructure _output_get_6)) (.currentxp (Variables|/Game/MAIN/PetSystem/Pets/Parent/Pet_Parent_BP.Pet_Parent_BP_C|GetPetStructure _output_get_6)) (.neededxp (Variables|/Game/MAIN/PetSystem/Pets/Parent/Pet_Parent_BP.Pet_Parent_BP_C|GetPetStructure _output_get_6))))
            (Variables|/Game/MAIN/PetSystem/Pets/Parent/Pet_Parent_BP.Pet_Parent_BP_C|SetIsHostile _output_get_6 true)
            (CallFunction|SetEnemyScales)))
        (else
          (Variables|Default|GetSpawnedPokemon
            (:then)
            (:else
              (bind _returnvalue_4 (AI|SpawnAIFromClass (Utilities|Array|Get(acopy) (Variables|Default|GetGhostlyCommonSpawns) (Math|Random|RandomIntegerinRange 0 2)) 0 (Transformation|GetWorldLocation (Variables|Default|GetWildSpawnPoint)) "0, 0, 0" true))
              (bind _output_get_7 (Variables|Default|SetSpawnedPokemon _returnvalue_4))
              (bind _aspet_parent_bp_4 (Utilities|Casting|CastToPet_Parent_BP _output_get_7))
              (bind _output_get_8 (Variables|Default|SetSpawnedDynamaxPokemon _aspet_parent_bp_4))
              (Transformation|SetActorScale3D _output_get_8 (Variables|Default|GetDynamaxScale))
              (Variables|/Script/Engine.CharacterMovementComponent|SetMaxWalkSpeed (Variables|/Script/Engine.Character|GetCharacterMovement _output_get_8) (Variables|Default|GetMaxDynamaxWalkSpeed))
              (Variables|/Game/MAIN/PetSystem/Pets/Parent/Pet_Parent_BP.Pet_Parent_BP_C|SetPetStructure _output_get_8 (Utilities|Struct|MakePoStructure (.name (Variables|/Game/MAIN/PetSystem/Pets/Parent/Pet_Parent_BP.Pet_Parent_BP_C|GetPetStructure _output_get_8)) (.isstackable (Variables|/Game/MAIN/PetSystem/Pets/Parent/Pet_Parent_BP.Pet_Parent_BP_C|GetPetStructure _output_get_8)) (.thumbnail (Variables|/Game/MAIN/PetSystem/Pets/Parent/Pet_Parent_BP.Pet_Parent_BP_C|GetPetStructure _output_get_8)) (.maxstacksize (Variables|/Game/MAIN/PetSystem/Pets/Parent/Pet_Parent_BP.Pet_Parent_BP_C|GetPetStructure _output_get_8)) (.isconsumable (Variables|/Game/MAIN/PetSystem/Pets/Parent/Pet_Parent_BP.Pet_Parent_BP_C|GetPetStructure _output_get_8)) (.description (Variables|/Game/MAIN/PetSystem/Pets/Parent/Pet_Parent_BP.Pet_Parent_BP_C|GetPetStructure _output_get_8)) (.pokédexno (Variables|/Game/MAIN/PetSystem/Pets/Parent/Pet_Parent_BP.Pet_Parent_BP_C|GetPetStructure _output_get_8)) (.species (Variables|/Game/MAIN/PetSystem/Pets/Parent/Pet_Parent_BP.Pet_Parent_BP_C|GetPetStructure _output_get_8)) (.class (Variables|/Game/MAIN/PetSystem/Pets/Parent/Pet_Parent_BP.Pet_Parent_BP_C|GetPetStructure _output_get_8)) (.pettag (Variables|/Game/MAIN/PetSystem/Pets/Parent/Pet_Parent_BP.Pet_Parent_BP_C|GetPetStructure _output_get_8)) (.pettype (Variables|/Game/MAIN/PetSystem/Pets/Parent/Pet_Parent_BP.Pet_Parent_BP_C|GetPetStructure _output_get_8)) (.pettype2 (Variables|/Game/MAIN/PetSystem/Pets/Parent/Pet_Parent_BP.Pet_Parent_BP_C|GetPetStructure _output_get_8)) (.raretype (Variables|/Game/MAIN/PetSystem/Pets/Parent/Pet_Parent_BP.Pet_Parent_BP_C|GetPetStructure _output_get_8)) (.nature (Variables|/Game/MAIN/PetSystem/Pets/Parent/Pet_Parent_BP.Pet_Parent_BP_C|GetPetStructure _output_get_8)) (.ivs (Variables|/Game/MAIN/PetSystem/Pets/Parent/Pet_Parent_BP.Pet_Parent_BP_C|GetPetStructure _output_get_8)) (.evs (Variables|/Game/MAIN/PetSystem/Pets/Parent/Pet_Parent_BP.Pet_Parent_BP_C|GetPetStructure _output_get_8)) (.cannotbepickedup (Variables|/Game/MAIN/PetSystem/Pets/Parent/Pet_Parent_BP.Pet_Parent_BP_C|GetPetStructure _output_get_8)) (.trainerownedby (Variables|/Game/MAIN/PetSystem/Pets/Parent/Pet_Parent_BP.Pet_Parent_BP_C|GetPetStructure _output_get_8)) (.cost (Variables|/Game/MAIN/PetSystem/Pets/Parent/Pet_Parent_BP.Pet_Parent_BP_C|GetPetStructure _output_get_8)) (.level (Variables|/Game/MAIN/PetSystem/Pets/Parent/Pet_Parent_BP.Pet_Parent_BP_C|GetPetStructure _output_get_8)) (+ (.currenthealth (Variables|/Game/MAIN/PetSystem/Pets/Parent/Pet_Parent_BP.Pet_Parent_BP_C|GetPetStructure _output_get_8)) 100) (+ (.maxhealth (Variables|/Game/MAIN/PetSystem/Pets/Parent/Pet_Parent_BP.Pet_Parent_BP_C|GetPetStructure _output_get_8)) 100) (.mindamage (Variables|/Game/MAIN/PetSystem/Pets/Parent/Pet_Parent_BP.Pet_Parent_BP_C|GetPetStructure _output_get_8)) (.maxdamage (Variables|/Game/MAIN/PetSystem/Pets/Parent/Pet_Parent_BP.Pet_Parent_BP_C|GetPetStructure _output_get_8)) (.currentmana (Variables|/Game/MAIN/PetSystem/Pets/Parent/Pet_Parent_BP.Pet_Parent_BP_C|GetPetStructure _output_get_8)) (.maxmana (Variables|/Game/MAIN/PetSystem/Pets/Parent/Pet_Parent_BP.Pet_Parent_BP_C|GetPetStructure _output_get_8)) (.happyness (Variables|/Game/MAIN/PetSystem/Pets/Parent/Pet_Parent_BP.Pet_Parent_BP_C|GetPetStructure _output_get_8)) false (.isdead (Variables|/Game/MAIN/PetSystem/Pets/Parent/Pet_Parent_BP.Pet_Parent_BP_C|GetPetStructure _output_get_8)) (.issummoned (Variables|/Game/MAIN/PetSystem/Pets/Parent/Pet_Parent_BP.Pet_Parent_BP_C|GetPetStructure _output_get_8)) true (.isattacking (Variables|/Game/MAIN/PetSystem/Pets/Parent/Pet_Parent_BP.Pet_Parent_BP_C|GetPetStructure _output_get_8)) (.isusingability1 (Variables|/Game/MAIN/PetSystem/Pets/Parent/Pet_Parent_BP.Pet_Parent_BP_C|GetPetStructure _output_get_8)) (.isusingability2 (Variables|/Game/MAIN/PetSystem/Pets/Parent/Pet_Parent_BP.Pet_Parent_BP_C|GetPetStructure _output_get_8)) (.isusingability3 (Variables|/Game/MAIN/PetSystem/Pets/Parent/Pet_Parent_BP.Pet_Parent_BP_C|GetPetStructure _output_get_8)) (.isusingability4 (Variables|/Game/MAIN/PetSystem/Pets/Parent/Pet_Parent_BP.Pet_Parent_BP_C|GetPetStructure _output_get_8)) (.isshiny (Variables|/Game/MAIN/PetSystem/Pets/Parent/Pet_Parent_BP.Pet_Parent_BP_C|GetPetStructure _output_get_8)) (.ismetallic (Variables|/Game/MAIN/PetSystem/Pets/Parent/Pet_Parent_BP.Pet_Parent_BP_C|GetPetStructure _output_get_8)) (.isghostly (Variables|/Game/MAIN/PetSystem/Pets/Parent/Pet_Parent_BP.Pet_Parent_BP_C|GetPetStructure _output_get_8)) (.petsize (Variables|/Game/MAIN/PetSystem/Pets/Parent/Pet_Parent_BP.Pet_Parent_BP_C|GetPetStructure _output_get_8)) (.issellable (Variables|/Game/MAIN/PetSystem/Pets/Parent/Pet_Parent_BP.Pet_Parent_BP_C|GetPetStructure _output_get_8)) (.canevolve (Variables|/Game/MAIN/PetSystem/Pets/Parent/Pet_Parent_BP.Pet_Parent_BP_C|GetPetStructure _output_get_8)) (.hasevolved (Variables|/Game/MAIN/PetSystem/Pets/Parent/Pet_Parent_BP.Pet_Parent_BP_C|GetPetStructure _output_get_8)) (.evolvesinto (Variables|/Game/MAIN/PetSystem/Pets/Parent/Pet_Parent_BP.Pet_Parent_BP_C|GetPetStructure _output_get_8)) (.currentxp (Variables|/Game/MAIN/PetSystem/Pets/Parent/Pet_Parent_BP.Pet_Parent_BP_C|GetPetStructure _output_get_8)) (.neededxp (Variables|/Game/MAIN/PetSystem/Pets/Parent/Pet_Parent_BP.Pet_Parent_BP_C|GetPetStructure _output_get_8))))
              (Variables|/Game/MAIN/PetSystem/Pets/Parent/Pet_Parent_BP.Pet_Parent_BP_C|SetIsHostile _output_get_8 true)
              (CallFunction|SetEnemyScales))))))))

(event Custom|CleanupPokeden
  (bind _spawneddynamaxpokemon (Variables|Default|GetSpawnedDynamaxPokemon)
    (:then
      (if (.isdead (Variables|/Game/MAIN/PetSystem/Pets/Parent/Pet_Parent_BP.Pet_Parent_BP_C|GetPetStructure _spawneddynamaxpokemon))
        (Utilities|FlowControl|DoOnce false :!label _label
          (:Completed
            (bind _asrpg_game_mode (Utilities|Casting|CastToRPG_GameMode (Game|GetGameMode)))
            (Default|StopDenBattleMusic _asrpg_game_mode)
            (Default|PlayRouteMusic _asrpg_game_mode)
            (Audio|PlaySound2D "/Game/MAIN/Pokemon/Sound/DynamaxRoar_Cue.DynamaxRoar_Cue" 1.0 1.0 0.0 0 0)
            (bind _playerreference (Variables|Default|GetPlayerReference)
              (:then
                (bind _toggledpet (Variables|/Game/MAIN/Blueprints/Player/MasterCharacter_BP.MasterCharacter_BP_C|GetToggledPet _playerreference)
                  (:then
                    (Transformation|SetActorScale3D _toggledpet "1.000000,1.000000,1.000000")
                    (Variables|/Script/Engine.CharacterMovementComponent|SetMaxWalkSpeed (Variables|/Script/Engine.Character|GetCharacterMovement _toggledpet) 6e+02))
                  (:else
                    _))
                (Variables|Default|SetIsEmpty true)
                (Rendering|SetVisibility (Variables|Default|GetBeam) false false)
                (CallFunction|ResetPlayerPokemonHealthtoNormal))
              (:else))))
        (else
          (goto _label Reset))))
    (:else
      (goto _label Reset))))

(event Custom|SetPlayerPokemonScales
  (bind _toggledpet (Variables|/Game/MAIN/Blueprints/Player/MasterCharacter_BP.MasterCharacter_BP_C|GetToggledPet (stale EventInteract _asmaster_character_bp))
    (:then
      (Variables|/Game/MAIN/PetSystem/Pets/Parent/Pet_Parent_BP.Pet_Parent_BP_C|SetContactHitLengh _toggledpet (Variables|Default|GetDynamaxPokemonContactHitLengh))
      (Variables|/Game/MAIN/PetSystem/Pets/Parent/Pet_Parent_BP.Pet_Parent_BP_C|SetContactHitScale _toggledpet (Variables|Default|GetDynamaxPokemonContactHitScale))
      (Variables|/Game/MAIN/PetSystem/Pets/Parent/Pet_Parent_BP.Pet_Parent_BP_C|SetDistanceHitLengh _toggledpet (Variables|Default|GetDynamaxPokemonDistanceHitLengh))
      (Variables|/Game/MAIN/PetSystem/Pets/Parent/Pet_Parent_BP.Pet_Parent_BP_C|SetDistanceHitScale _toggledpet (Variables|Default|GetDynamaxPokemonDistanceHitScale))
      (Variables|/Game/MAIN/PetSystem/Pets/Parent/Pet_Parent_BP.Pet_Parent_BP_C|SetContactHitParticleScale _toggledpet (Variables|Default|GetDynamaxPokemonHitParticleScale))
      (Variables|/Game/MAIN/PetSystem/Pets/Parent/Pet_Parent_BP.Pet_Parent_BP_C|SetDistanceHitParticleScale _toggledpet (Variables|Default|GetDynamaxPokemonDistanceHitParticleScale))
      (Variables|/Game/MAIN/PetSystem/Pets/Parent/Pet_Parent_BP.Pet_Parent_BP_C|SetPidgeyGustParticleScale _toggledpet (Variables|Default|GetDynamaxPokemonPidgeyGustParticleScale))
      (Variables|/Script/Engine.SpringArmComponent|SetTargetArmLength (Variables|/Game/MAIN/PetSystem/Pets/Parent/Pet_Parent_BP.Pet_Parent_BP_C|GetCameraBoom _toggledpet) 7e+03)
      (Variables|/Game/MAIN/PetSystem/Pets/Parent/Pet_Parent_BP.Pet_Parent_BP_C|SetZoomInteval _toggledpet 5e+02)
      (Variables|/Game/MAIN/PetSystem/Pets/Parent/Pet_Parent_BP.Pet_Parent_BP_C|SetContactAttackMinDmgMultiplier _toggledpet (Variables|Default|GetDynamaxContactAttackMinDmgMultiplier))
      (Variables|/Game/MAIN/PetSystem/Pets/Parent/Pet_Parent_BP.Pet_Parent_BP_C|SetContactAttackMaxDmgMultiplier _toggledpet (Variables|Default|GetDynamaxContactAttackMaxDmgMultiplier))
      (Variables|/Game/MAIN/PetSystem/Pets/Parent/Pet_Parent_BP.Pet_Parent_BP_C|SetDistanceAttackMinDmgMultiplier _toggledpet (Variables|Default|GetDynamaxDistanceAttackMinDmgMultiplier))
      (Variables|/Game/MAIN/PetSystem/Pets/Parent/Pet_Parent_BP.Pet_Parent_BP_C|SetDistanceAttackMaxDmgMultiplier _toggledpet (Variables|Default|GetDynamaxDistanceAttackMaxDmgMultiplier))
      (CallFunction|ControlPokemoninDen))
    (:else)))

(event Custom|SetEnemyScales
  (bind _spawneddynamaxpokemon (Variables|Default|GetSpawnedDynamaxPokemon)
    (:then
      (Variables|/Game/MAIN/PetSystem/Pets/Parent/Pet_Parent_BP.Pet_Parent_BP_C|SetContactHitLengh _spawneddynamaxpokemon (Variables|Default|GetDynamaxPokemonContactHitLengh))
      (Variables|/Game/MAIN/PetSystem/Pets/Parent/Pet_Parent_BP.Pet_Parent_BP_C|SetContactHitScale _spawneddynamaxpokemon (Variables|Default|GetDynamaxPokemonContactHitScale))
      (Variables|/Game/MAIN/PetSystem/Pets/Parent/Pet_Parent_BP.Pet_Parent_BP_C|SetDistanceHitLengh _spawneddynamaxpokemon (Variables|Default|GetDynamaxPokemonDistanceHitLengh))
      (Variables|/Game/MAIN/PetSystem/Pets/Parent/Pet_Parent_BP.Pet_Parent_BP_C|SetDistanceHitScale _spawneddynamaxpokemon (Variables|Default|GetDynamaxPokemonDistanceHitScale))
      (Variables|/Game/MAIN/PetSystem/Pets/Parent/Pet_Parent_BP.Pet_Parent_BP_C|SetContactHitParticleScale _spawneddynamaxpokemon (Variables|Default|GetDynamaxPokemonHitParticleScale))
      (Variables|/Game/MAIN/PetSystem/Pets/Parent/Pet_Parent_BP.Pet_Parent_BP_C|SetDistanceHitParticleScale _spawneddynamaxpokemon (Variables|Default|GetDynamaxPokemonDistanceHitParticleScale))
      (Variables|/Game/MAIN/PetSystem/Pets/Parent/Pet_Parent_BP.Pet_Parent_BP_C|SetPidgeyGustParticleScale _spawneddynamaxpokemon (Variables|Default|GetDynamaxPokemonPidgeyGustParticleScale))
      (Variables|/Game/MAIN/PetSystem/Pets/Parent/Pet_Parent_BP.Pet_Parent_BP_C|SetContactAttackMinDmgMultiplier _spawneddynamaxpokemon (Variables|Default|GetDynamaxContactAttackMinDmgMultiplier))
      (Variables|/Game/MAIN/PetSystem/Pets/Parent/Pet_Parent_BP.Pet_Parent_BP_C|SetContactAttackMaxDmgMultiplier _spawneddynamaxpokemon (Variables|Default|GetDynamaxContactAttackMaxDmgMultiplier))
      (Variables|/Game/MAIN/PetSystem/Pets/Parent/Pet_Parent_BP.Pet_Parent_BP_C|SetDistanceAttackMinDmgMultiplier _spawneddynamaxpokemon (Variables|Default|GetDynamaxDistanceAttackMinDmgMultiplier))
      (Variables|/Game/MAIN/PetSystem/Pets/Parent/Pet_Parent_BP.Pet_Parent_BP_C|SetDistanceAttackMaxDmgMultiplier _spawneddynamaxpokemon (Variables|Default|GetDynamaxDistanceAttackMaxDmgMultiplier)))
    (:else)))

(event Custom|CleanupDenRecall
  (if (Variables|Default|GetInDen)
    (bind _spawneddynamaxpokemon (Variables|Default|GetSpawnedDynamaxPokemon)
      (:then
        (Actor|DestroyActor _spawneddynamaxpokemon))
      (:else
        _))
    (Variables|Default|SetInDen false)
    (bind _asrpg_game_mode (Utilities|Casting|CastToRPG_GameMode (Game|GetGameMode)))
    (Default|StopDenBattleMusic _asrpg_game_mode)
    (Default|PlayRouteMusic _asrpg_game_mode)
    (Audio|PlaySound2D "/Game/MAIN/Pokemon/Sound/DynamaxRoar_Cue.DynamaxRoar_Cue" 1.0 1.0 0.0 0 0)
    (bind _playerreference (Variables|Default|GetPlayerReference)
      (:then
        (bind _toggledpet (Variables|/Game/MAIN/Blueprints/Player/MasterCharacter_BP.MasterCharacter_BP_C|GetToggledPet _playerreference)
          (:then
            (Transformation|SetActorScale3D _toggledpet "1.000000,1.000000,1.000000")
            (Variables|/Script/Engine.CharacterMovementComponent|SetMaxWalkSpeed (Variables|/Script/Engine.Character|GetCharacterMovement _toggledpet) 6e+02))
          (:else
            _))
        (Variables|Default|SetIsEmpty true)
        (Rendering|SetVisibility (Variables|Default|GetBeam) false false)
        (CallFunction|ResetPlayerPokemonHealthtoNormal))
      (:else))))

(event EventBeginPlay
  (bind _asmaster_character_bp (Utilities|Casting|CastToMasterCharacter_BP (Game|GetPlayerCharacter 0)))
  (Variables|Default|SetPlayerReference _asmaster_character_bp)
  (if (Math|Random|RandomBoolwithWeight 0.6)
    (Variables|Default|SetIsEmpty true)
    (Rendering|SetVisibility (Variables|Default|GetBeam) false false)
    (else
      (Variables|Default|SetIsEmpty false)
      (Rendering|SetVisibility (Variables|Default|GetBeam) true false))))

(event Collision|EventActorBeginOverlap
  (params (OtherActor :type Actor%20Object%20Reference)))

(event EventTick
  (params (DeltaSeconds :type Float%20%28single-precision%29))
  (Utilities|FlowControl|Sequence
    (:then_0
      (Utilities|FlowControl|Delay 7e+02)
      (Utilities|FlowControl|DoOnce false :!label _label
        (:Completed
          (if (Math|Random|RandomBoolwithWeight 0.5)
            (Variables|Default|SetIsEmpty true)
            (Rendering|SetVisibility (Variables|Default|GetBeam) false false)
            (goto _label Reset)
            (else
              (Variables|Default|SetIsEmpty false)
              (Rendering|SetVisibility (Variables|Default|GetBeam) true false)
              (goto _label Reset))))))
    (:then_1
      (bind _spawneddynamaxpokemon (Variables|Default|GetSpawnedDynamaxPokemon)
        (:then
          (if (.isdead (Variables|/Game/MAIN/PetSystem/Pets/Parent/Pet_Parent_BP.Pet_Parent_BP_C|GetPetStructure _spawneddynamaxpokemon))
            (Utilities|FlowControl|DoOnce false :!label _label_2
              (:Completed
                (bind _asrpg_game_mode (Utilities|Casting|CastToRPG_GameMode (Game|GetGameMode)))
                (Default|StopDenBattleMusic _asrpg_game_mode)
                (Default|PlayRouteMusic _asrpg_game_mode)
                (Audio|PlaySound2D "/Game/MAIN/Pokemon/Sound/DynamaxRoar_Cue.DynamaxRoar_Cue" 1.0 1.0 0.0 0 0)
                (bind _playerreference (Variables|Default|GetPlayerReference)
                  (:then
                    (bind _toggledpet (Variables|/Game/MAIN/Blueprints/Player/MasterCharacter_BP.MasterCharacter_BP_C|GetToggledPet _playerreference)
                      (:then
                        (Transformation|SetActorScale3D _toggledpet "1.000000,1.000000,1.000000")
                        (Variables|/Script/Engine.CharacterMovementComponent|SetMaxWalkSpeed (Variables|/Script/Engine.Character|GetCharacterMovement _toggledpet) 6e+02))
                      (:else
                        _))
                    (Variables|Default|SetIsEmpty true)
                    (Rendering|SetVisibility (Variables|Default|GetBeam) false false)
                    (CallFunction|ResetPlayerPokemonHealthtoNormal))
                  (:else))))
            (else
              (goto _label_2 Reset))))
        (:else
          (goto _label_2 Reset))))))

(event EventInteract
  (params (Interacter :type Actor%20Object%20Reference))
  (bind _asmaster_character_bp (Utilities|Casting|CastToMasterCharacter_BP Interacter))
  (if (Variables|Default|GetIsEmpty)
    (Default|ToggleEmptyDenUI _asmaster_character_bp)
    (elif (== (Variables|/Game/MAIN/Blueprints/Player/MasterCharacter_BP.MasterCharacter_BP_C|GetToggledPet _asmaster_character_bp) 0)
      (Default|ToggleSummonFirstforDen _asmaster_character_bp)
      (else
        (bind _toggledpet (Variables|/Game/MAIN/Blueprints/Player/MasterCharacter_BP.MasterCharacter_BP_C|GetToggledPet _asmaster_character_bp)
          (:then
            (Variables|Default|GetLoadingUI
              (:then
                _)
              (:else
                (bind _returnvalue (UserInterface|CreateWidget "/Game/MAIN/UI/Loading_UI.Loading_UI_C"))
                (bind _output_get (Variables|Default|SetLoadingUI _returnvalue))
                (UserInterface|Viewport|AddtoViewport _output_get 0)
                (Variables|Default|SetInDen true)))
            (CallFunction|SaveHealthOfPlayerPokemon))
          (:else
            (Default|ToggleSummonFirstforDen _asmaster_character_bp)))))))

(fn ConstructionScript)