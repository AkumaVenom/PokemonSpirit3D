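; Pokemon spawner, named for Charizard AI battles, that keeps one hostile Pokemon alive at its spawn point.
; Each Tick checks the stored Pokemon and, if it is invalid, spawns a replacement from CommonSpawns; the random index always resolves to the first entry.
; The spawn is cast to Pet_Parent_BP, stored and flagged hostile and able to attack.
; A DoOnce gates the check, resetting after each successful pass.
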(event Collision|EventActorBeginOverlap
  (params (OtherActor :type Actor%20Object%20Reference)))

(event EventTick
  (params (DeltaSeconds :type Float%20%28single-precision%29))
  (Utilities|FlowControl|DoOnce false :!label _label
    (:Completed
      (Variables|Default|GetSpawnedPokemonBP
        (:then
          (goto _label Reset))
        (:else
          (bind _returnvalue (AI|SpawnAIFromClass (Utilities|Array|Get(acopy) (Variables|Default|GetCommonSpawns) (Math|Random|RandomIntegerinRange 0 0)) 0 (Transformation|GetWorldLocation (Variables|Default|GetSpawnPoint)) "0, 0, 0" true))
          (bind _aspet_parent_bp (Utilities|Casting|CastToPet_Parent_BP _returnvalue))
          (bind _output_get (Variables|Default|SetSpawnedPokemonBP _aspet_parent_bp))
          (Variables|/Game/MAIN/PetSystem/Pets/Parent/Pet_Parent_BP.Pet_Parent_BP_C|SetIsHostile _output_get true)
          (Variables|/Game/MAIN/PetSystem/Pets/Parent/Pet_Parent_BP.Pet_Parent_BP_C|SetCanAttack _output_get true)
          (goto _label Reset))))))

(fn ConstructionScript)