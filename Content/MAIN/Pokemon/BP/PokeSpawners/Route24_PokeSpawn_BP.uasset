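; Route 24 Pokémon spawner that spawns a wild Pokémon when the player character or a player-controlled pet overlaps its Sphere.
; Nested weighted rolls select the common, uncommon or legendary tier, with legendary as the fallback when both rolls fail.
; A class from that tier's array spawns as AI at SpawnPoint, unless the previously spawned Pokémon is still valid, limiting the spawner to one at a time.
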(event OnComponentBeginOverlap(Sphere)
  (params (OverlappedComponent :type Primitive%20Component%20Object%20Reference) (OtherActor :type Actor%20Object%20Reference) (OtherComp :type Primitive%20Component%20Object%20Reference) (OtherBodyIndex :type Integer) (bFromSweep :type Boolean) (SweepResult :type Hit%20Result%20Structure%20%28by%20ref%29))
  (Utilities|Casting|CastToMasterCharacter_BP OtherActor
    (:then
      (if (Math|Random|RandomBoolwithWeight (Variables|Default|GetCommonSpawnRate)) :!label _label
        (Utilities|FlowControl|DoOnce false :!label _label_2
          (:Completed
            (Variables|Default|GetSpawnedPokemon
              (:then
                (goto _label_2 Reset))
              (:else
                (bind _returnvalue (AI|SpawnAIFromClass (Utilities|Array|Get(acopy) (Variables|Default|GetCommonSpawns) (Math|Random|RandomIntegerinRange 0 3)) 0 (Transformation|GetWorldLocation (Variables|Default|GetSpawnPoint)) "0, 0, 0" true))
                (Variables|Default|SetSpawnedPokemon _returnvalue)
                (goto _label_2 Reset)))))
        (elif (Math|Random|RandomBoolwithWeight (Variables|Default|GetUncommonSpawnRate))
          (Utilities|FlowControl|DoOnce false :!label _label_3
            (:Completed
              (Variables|Default|GetSpawnedPokemon
                (:then
                  (goto _label_3 Reset))
                (:else
                  (bind _returnvalue_2 (AI|SpawnAIFromClass (Utilities|Array|Get(acopy) (Variables|Default|GetUncommonSpawns) (Math|Random|RandomIntegerinRange 0 2)) 0 (Transformation|GetWorldLocation (Variables|Default|GetSpawnPoint)) "0, 0, 0" true))
                  (Variables|Default|SetSpawnedPokemon _returnvalue_2)
                  (goto _label_3 Reset)))))
          (else
            (Utilities|FlowControl|DoOnce false :!label _label_4
              (:Completed
                (Variables|Default|GetSpawnedPokemon
                  (:then
                    (goto _label_4 Reset))
                  (:else
                    (bind _returnvalue_3 (AI|SpawnAIFromClass (Utilities|Array|Get(acopy) (Variables|Default|GetLegendarySpawns) (Math|Random|RandomIntegerinRange 0 0)) 0 (Transformation|GetWorldLocation (Variables|Default|GetSpawnPoint)) "0, 0, 0" true))
                    (Variables|Default|SetSpawnedPokemon _returnvalue_3)
                    (goto _label_4 Reset)))))))))
    (:CastFailed
      (bind _aspet_parent_bp (Utilities|Casting|CastToPet_Parent_BP OtherActor))
      (if (Pawn|IsPlayerControlled _aspet_parent_bp)
        (goto _label)))))

(event EventBeginPlay
  (bind _outactors (Actor|GetAllActorsOfClass "/Game/MAIN/Blueprints/Player/MasterCharacter_BP.MasterCharacter_BP_C"))
  (Variables|Default|SetPlayerRef (Utilities|Array|Get(acopy) _outactors)))

(event Collision|EventActorBeginOverlap
  (params (OtherActor :type Actor%20Object%20Reference)))

(fn ConstructionScript)