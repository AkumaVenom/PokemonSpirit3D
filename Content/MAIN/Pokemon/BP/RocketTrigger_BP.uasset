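; RocketTrigger_BP is a trigger actor that stages a Team Rocket moment with theme music and a camera cut when the player walks in.
; When the MasterCharacter overlaps its sphere and no theme sound exists yet, it creates and plays the 2D theme, then blends the view to itself.
; After a delay it blends the camera back to the player reference cached on BeginPlay.
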(event OnComponentBeginOverlap(Sphere)
  (params (OverlappedComponent :type Primitive%20Component%20Object%20Reference) (OtherActor :type Actor%20Object%20Reference) (OtherComp :type Primitive%20Component%20Object%20Reference) (OtherBodyIndex :type Integer) (bFromSweep :type Boolean) (SweepResult :type Hit%20Result%20Structure%20%28by%20ref%29))
  (Utilities|Casting|CastToMasterCharacter_BP OtherActor)
  (Variables|Default|GetRocketTheme
    (:then)
    (:else
      (bind _returnvalue (Audio|CreateSound2D "/Game/MAIN/Pokemon/Music/teamRocketTheme_Cue.teamRocketTheme_Cue" 2.0 1.0 0.0 0))
      (bind _output_get (Variables|Default|SetRocketTheme _returnvalue))
      (Audio|Components|Audio|Play _output_get 0.0)
      (Game|Player|SetViewTargetwithBlend (Game|GetPlayerController 0) self 2.0 "VTBlend_Linear" 0.0 false)
      (Utilities|FlowControl|Delay 1e+01)
      (bind _playerreference (Variables|Default|GetPlayerReference)
        (:then
          (Game|Player|SetViewTargetwithBlend (Game|GetPlayerController 0) _playerreference 2.0 "VTBlend_Linear" 0.0 false))
        (:else)))))

(event EventBeginPlay
  (bind _asmaster_character_bp (Utilities|Casting|CastToMasterCharacter_BP (Game|GetPlayerCharacter 0)))
  (Variables|Default|SetPlayerReference _asmaster_character_bp))

(event Collision|EventActorBeginOverlap
  (params (OtherActor :type Actor%20Object%20Reference)))

(event EventTick
  (params (DeltaSeconds :type Float%20%28single-precision%29)))

(fn ConstructionScript)