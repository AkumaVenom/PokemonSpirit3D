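; Parent Blueprint for NPCs that roll loot on spawn and can be looted by the player once dead.
; On BeginPlay it caches the first MasterCharacter_BP and fills its InventoryComponent from a weighted random pick of empty, herb or gem drop tables.
; Interacting at zero health toggles that inventory.
; Tick destroys it beyond RadiusToDespawn from the player, or after a random post-death delay, toggling any open inventory first.
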(event EventBeginPlay
  (bind _outactors (Actor|GetAllActorsOfClass "/Game/MAIN/Blueprints/Player/MasterCharacter_BP.MasterCharacter_BP_C"))
  (Variables|Default|SetPlayerReference (Utilities|Array|Get(acopy) _outactors))
  (CallFunction|CalculateLoot))

(event EventTick
  (params (DeltaSeconds :type Float%20%28single-precision%29))
  (bind _inventorycomponent (Variables|Default|GetInventoryComponent))
  (Utilities|FlowControl|Sequence
    (:then_0
      (if (> (Transformation|GetDistanceTo self (Variables|Default|GetPlayerReference)) (Variables|Default|GetRadiusToDespawn))
        (Utilities|FlowControl|DoOnce false
          (:Completed
            (Actor|DestroyActor)))))
    (:then_1
      (if (<= (Variables|Default|GetCurrentHealth) 0)
        (Utilities|FlowControl|DoOnce false
          (:Completed
            (Utilities|FlowControl|Delay (Math|Random|RandomFloatinRange 15.0 25.0))
            (if (Variables|/Game/MAIN/InventorySystem/InventoryComponent.InventoryComponent_C|GetInventoryToggled _inventorycomponent)
              (Default|ToggleInventoryON _inventorycomponent))
            (Actor|DestroyActor)))))))

(event EventInteract
  (params (Interacter :type Actor%20Object%20Reference))
  (Utilities|Casting|CastToMasterCharacter_BP Interacter)
  (if (<= (Variables|Default|GetCurrentHealth) 0)
    (Default|ToggleInventoryON (Variables|Default|GetInventoryComponent))))

(fn ConstructionScript)

(fn CalculateLoot
  (if (Math|Random|RandomBoolwithWeight 0.5)
    (for (_array_element _array_index) (Variables|Default|GetNoneDropTable)
      (Utilities|Array|SetArrayElem (Variables|/Game/MAIN/InventorySystem/InventoryComponent.InventoryComponent_C|GetInventory (Variables|Default|GetInventoryComponent)) _array_index _array_element))
    (elif (Math|Random|RandomBoolwithWeight 0.51)
      (switch int (Math|Random|RandomIntegerinRange 0 2)
        (:0
          (for (_array_element_2 _array_index_2) (Variables|Default|GetHP_HerbDropTable)
            (Utilities|Array|SetArrayElem (Variables|/Game/MAIN/InventorySystem/InventoryComponent.InventoryComponent_C|GetInventory (Variables|Default|GetInventoryComponent)) _array_index_2 _array_element_2)))
        (:1
          (for (_array_element_3 _array_index_3) (Variables|Default|GetMP_HerbDropTable)
            (Utilities|Array|SetArrayElem (Variables|/Game/MAIN/InventorySystem/InventoryComponent.InventoryComponent_C|GetInventory (Variables|Default|GetInventoryComponent)) _array_index_3 _array_element_3)))
        (:2
          (for (_array_element_4 _array_index_4) (Variables|Default|GetHP_MP_HERBS_DroptTable)
            (Utilities|Array|SetArrayElem (Variables|/Game/MAIN/InventorySystem/InventoryComponent.InventoryComponent_C|GetInventory (Variables|Default|GetInventoryComponent)) _array_index_4 _array_element_4))))
      (else
        (switch int (Math|Random|RandomIntegerinRange 0 2)
          (:0
            (for (_array_element_5 _array_index_5) (Variables|Default|GetGemDropTable1)
              (Utilities|Array|SetArrayElem (Variables|/Game/MAIN/InventorySystem/InventoryComponent.InventoryComponent_C|GetInventory (Variables|Default|GetInventoryComponent)) _array_index_5 _array_element_5)))
          (:1
            (for (_array_element_6 _array_index_6) (Variables|Default|GetGemDropTable2)
              (Utilities|Array|SetArrayElem (Variables|/Game/MAIN/InventorySystem/InventoryComponent.InventoryComponent_C|GetInventory (Variables|Default|GetInventoryComponent)) _array_index_6 _array_element_6)))
          (:2
            (for (_array_element_7 _array_index_7) (Variables|Default|GetGemDropTable3)
              (Utilities|Array|SetArrayElem (Variables|/Game/MAIN/InventorySystem/InventoryComponent.InventoryComponent_C|GetInventory (Variables|Default|GetInventoryComponent)) _array_index_7 _array_element_7))))))))