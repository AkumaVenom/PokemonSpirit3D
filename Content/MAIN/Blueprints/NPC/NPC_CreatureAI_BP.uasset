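; NPC creature AI that free-roams and, when hostile, chases and melee-attacks the player.
; Tick sends it to random reachable points after random delays until PawnSensing sees or hears the player character, which permanently stops roaming if hostile.
; A delayed loop reissues AIMoveTo toward the player while hostile and alive.
; On arrival it faces the player, line-traces forward and applies random damage with a slash effect unless the player is dodging.
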(event OnSeePawn(PawnSensing)
  (params (Pawn :type Pawn%20Object%20Reference))
  (bind _capsulecomponent (Variables|Default|GetCapsuleComponent))
  (bind _returnvalue (Transformation|GetWorldLocation _capsulecomponent))
  (Utilities|Casting|CastToMasterCharacter_BP Pawn)
  (if (Variables|Default|GetIsHostile)
    (if (not (Variables|Default|GetIsDead))
      (if (not (Variables|Default|GetIsAttacking))
        (Variables|Default|SetCanFreeRoam false)
        (Variables|/Script/Engine.CharacterMovementComponent|SetMaxWalkSpeed (Variables|Character|GetCharacterMovement) (Variables|Default|GetMaxWalkSpeedEnemySeen))
        (AI|AIMoveTo self "0, 0, 0" (Variables|Default|GetPlayerReference) 2e+01 false :!label _label
          (:then
            (Utilities|FlowControl|Delay 1.0)
            (if (Variables|Default|GetIsHostile) :!label _label_2
              (if (not (Variables|Default|GetIsDead))
                (goto _label))))
          (:OnSuccess
            (Transformation|SetActorRotation (Math|Rotator|MakeRotator 0.0 0.0 (.yaw (Math|Rotator|FindLookatRotation (Transformation|GetActorLocation self) (Transformation|GetActorLocation (Variables|Default|GetPlayerReference))))))
            (bind (_outhit _returnvalue_2) (Collision|LineTraceForObjects _returnvalue (+ _returnvalue (* (Math|Vector|GetForwardVector _capsulecomponent) 3e+02)) (Utilities|Array|MakeArray "ObjectTypeQuery3") false 0 "None"))
            (Variables|Default|SetIsAttacking true)
            (Variables|Default|SetHitLocation (.Location (Collision|BreakHitResult _outhit)))
            (Variables|Default|SetHitActor (.HitActor (Collision|BreakHitResult _outhit)))
            (if _returnvalue_2
              (bind _asmaster_character_bp (Utilities|Casting|CastToMasterCharacter_BP (Variables|Default|GetHitActor)))
              (if (Variables|/Game/MAIN/Blueprints/Player/MasterCharacter_BP.MasterCharacter_BP_C|GetIsDodging _asmaster_character_bp)
                _
                (else
                  (Variables|/Game/MAIN/Blueprints/Player/MasterCharacter_BP.MasterCharacter_BP_C|SetCurrentHealth _asmaster_character_bp (- (Variables|/Game/MAIN/Blueprints/Player/MasterCharacter_BP.MasterCharacter_BP_C|GetCurrentHealth _asmaster_character_bp) (Math|Random|RandomIntegerinRange (Variables|Default|GetMinimumDamage) (Variables|Default|GetMaxDamage))))
                  (Effects|SpawnEmitteratLocation "/Game/FXs/Impact/FX/Particle/Yellow/PS_GFXI_Red_Slash_02.PS_GFXI_Red_Slash_02" (Variables|Default|GetHitLocation))))
              (Utilities|FlowControl|Delay 1.0)
              (Variables|Default|SetIsAttacking false)
              (else
                (Utilities|FlowControl|Delay (Variables|Default|GetAttackAnimationLength))
                (Variables|Default|SetIsAttacking false))))
          (:OnFail
            (goto _label_2)))))))

(event OnHearNoise(PawnSensing)
  (params (Instigator :type Pawn%20Object%20Reference) (Location :type Vector%20%28by%20ref%29 :default "0, 0, 0") (Volume :type Float%20%28single-precision%29))
  (bind _capsulecomponent (Variables|Default|GetCapsuleComponent))
  (bind _returnvalue (Transformation|GetWorldLocation _capsulecomponent))
  (Utilities|Casting|CastToMasterCharacter_BP Instigator)
  (if (Variables|Default|GetIsHostile)
    (if (not (Variables|Default|GetIsDead))
      (if (not (Variables|Default|GetIsAttacking))
        (Variables|Default|SetCanFreeRoam false)
        (Variables|/Script/Engine.CharacterMovementComponent|SetMaxWalkSpeed (Variables|Character|GetCharacterMovement) (Variables|Default|GetMaxWalkSpeedEnemySeen))
        (AI|AIMoveTo self "0, 0, 0" (Variables|Default|GetPlayerReference) 2e+01 false :!label _label
          (:then
            (Utilities|FlowControl|Delay 1.0)
            (if (Variables|Default|GetIsHostile) :!label _label_2
              (if (not (Variables|Default|GetIsDead))
                (goto _label))))
          (:OnSuccess
            (Transformation|SetActorRotation (Math|Rotator|MakeRotator 0.0 0.0 (.yaw (Math|Rotator|FindLookatRotation (Transformation|GetActorLocation self) (Transformation|GetActorLocation (Variables|Default|GetPlayerReference))))))
            (bind (_outhit _returnvalue_2) (Collision|LineTraceForObjects _returnvalue (+ _returnvalue (* (Math|Vector|GetForwardVector _capsulecomponent) 3e+02)) (Utilities|Array|MakeArray "ObjectTypeQuery3") false 0 "None"))
            (Variables|Default|SetIsAttacking true)
            (Variables|Default|SetHitLocation (.Location (Collision|BreakHitResult _outhit)))
            (Variables|Default|SetHitActor (.HitActor (Collision|BreakHitResult _outhit)))
            (if _returnvalue_2
              (bind _asmaster_character_bp (Utilities|Casting|CastToMasterCharacter_BP (Variables|Default|GetHitActor)))
              (if (Variables|/Game/MAIN/Blueprints/Player/MasterCharacter_BP.MasterCharacter_BP_C|GetIsDodging _asmaster_character_bp)
                _
                (else
                  (Variables|/Game/MAIN/Blueprints/Player/MasterCharacter_BP.MasterCharacter_BP_C|SetCurrentHealth _asmaster_character_bp (- (Variables|/Game/MAIN/Blueprints/Player/MasterCharacter_BP.MasterCharacter_BP_C|GetCurrentHealth _asmaster_character_bp) (Math|Random|RandomIntegerinRange (Variables|Default|GetMinimumDamage) (Variables|Default|GetMaxDamage))))
                  (Effects|SpawnEmitteratLocation "/Game/FXs/Impact/FX/Particle/Yellow/PS_GFXI_Red_Slash_02.PS_GFXI_Red_Slash_02" (Variables|Default|GetHitLocation))))
              (Utilities|FlowControl|Delay 1.0)
              (Variables|Default|SetIsAttacking false)
              (else
                (Utilities|FlowControl|Delay (Variables|Default|GetAttackAnimationLength))
                (Variables|Default|SetIsAttacking false))))
          (:OnFail
            (goto _label_2)))))))

(event EventBeginPlay
  (|CallParentFunction) ; This node is disabled and will not be called.\nDrag off pins to build functionality.
)

(event Collision|EventActorBeginOverlap
  (params (OtherActor :type Actor%20Object%20Reference)))

(event EventTick
  (params (DeltaSeconds :type Float%20%28single-precision%29))
  (|CallParentFunction DeltaSeconds)
  (if (Variables|Default|GetCanFreeRoam)
    (Utilities|FlowControl|Delay (Math|Random|RandomFloatinRange 3.0 7.0))
    (Variables|/Script/Engine.CharacterMovementComponent|SetMaxWalkSpeed (Variables|Character|GetCharacterMovement) (Variables|Default|GetMaxWalkSpeedFreeRoam))
    (Variables|Default|SetIsMoving true)
    (AI|AIMoveTo self (.RandomLocation (AI|Navigation|GetRandomReachablePointinRadius (Transformation|GetActorLocation) 2e+03 0 0)) 0 5.0 false
      (:OnSuccess
        _)
      (:OnFail
        _))
    (Variables|Default|SetIsMoving false)))

(fn ConstructionScript
  (|CallParentFunction))