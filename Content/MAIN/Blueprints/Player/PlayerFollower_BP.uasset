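; Partner character that follows the player and can appear as one of seven companions, such as Red, May, Lillie or Lana.
; Each tick it uses AIMoveTo toward the MasterCharacter_BP found at BeginPlay, snapping to that player's PetSpawnPoint when it falls too far behind.
; Selection events set exclusive partner flags and swap mesh, anim class and scale.
; Shortly after BeginPlay, CalculatePartnerSkin applies the flagged skin, defaulting to Red.
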(event Custom|RedPartnerSelected
  (bind _mesh (Variables|Character|GetMesh))
  (Variables|Default|SetIsRedPartner true)
  (Variables|Default|SetIsSophoclesPartner false)
  (Variables|Default|SetIsMayPartner false)
  (Variables|Default|SetIsMallowPartner false)
  (Variables|Default|SetIsLilliePartner false)
  (Variables|Default|SetIsLanaPartner false)
  (Variables|Default|SetIsAcerolaPartner false)
  (Class|SkinnedMeshComponent|SetSkeletalMesh _mesh "/Game/MAIN/Pokemon/Trainers/REDv2/667.667" true)
  (Class|SkeletalMeshComponent|SetAnimClass _mesh "/Game/MAIN/Pokemon/Trainers/REDv2/RedFollowerAnimBP.RedFollowerAnimBP_C")
  (Transformation|SetRelativeScale3D _mesh "100.000000,100.000000,100.000000"))

(event Custom|SophoclesPartnerSelected
  (bind _mesh (Variables|Character|GetMesh))
  (Variables|Default|SetIsRedPartner false)
  (Variables|Default|SetIsSophoclesPartner true)
  (Variables|Default|SetIsMayPartner false)
  (Variables|Default|SetIsMallowPartner false)
  (Variables|Default|SetIsLilliePartner false)
  (Variables|Default|SetIsLanaPartner false)
  (Variables|Default|SetIsAcerolaPartner false)
  (Class|SkinnedMeshComponent|SetSkeletalMesh _mesh "/Game/MAIN/Pokemon/Trainers/Sophocles/665.665" true)
  (Class|SkeletalMeshComponent|SetAnimClass _mesh "/Game/MAIN/Pokemon/Trainers/Sophocles/SophoclesFollowerAnimBP.SophoclesFollowerAnimBP_C")
  (Transformation|SetRelativeScale3D _mesh "100.000000,100.000000,100.000000"))

(event Custom|MayPartnerSelected
  (bind _mesh (Variables|Character|GetMesh))
  (Variables|Default|SetIsRedPartner false)
  (Variables|Default|SetIsSophoclesPartner false)
  (Variables|Default|SetIsMayPartner true)
  (Variables|Default|SetIsMallowPartner false)
  (Variables|Default|SetIsLilliePartner false)
  (Variables|Default|SetIsLanaPartner false)
  (Variables|Default|SetIsAcerolaPartner false)
  (Class|SkinnedMeshComponent|SetSkeletalMesh _mesh "/Game/MAIN/Pokemon/Trainers/May/May_SK.May_SK" true)
  (Class|SkeletalMeshComponent|SetAnimClass _mesh "/Game/MAIN/Pokemon/Trainers/May/May_SKFollower_AnimBP.May_SKFollower_AnimBP_C")
  (Transformation|SetRelativeScale3D _mesh "1.170000,1.170000,1.170000"))

(event Custom|MallowPartnerSelected
  (bind _mesh (Variables|Character|GetMesh))
  (Variables|Default|SetIsRedPartner false)
  (Variables|Default|SetIsSophoclesPartner false)
  (Variables|Default|SetIsMayPartner false)
  (Variables|Default|SetIsMallowPartner true)
  (Variables|Default|SetIsLilliePartner false)
  (Variables|Default|SetIsLanaPartner false)
  (Variables|Default|SetIsAcerolaPartner false)
  (Class|SkinnedMeshComponent|SetSkeletalMesh _mesh "/Game/MAIN/Pokemon/Trainers/Mallow/664.664" true)
  (Class|SkeletalMeshComponent|SetAnimClass _mesh "/Game/MAIN/Pokemon/Trainers/Mallow/MallowFollowerAnimBP.MallowFollowerAnimBP_C")
  (Transformation|SetRelativeScale3D _mesh "100.000000,100.000000,100.000000"))

(event Custom|LilliePartnerSelected
  (bind _mesh (Variables|Character|GetMesh))
  (Variables|Default|SetIsRedPartner false)
  (Variables|Default|SetIsSophoclesPartner false)
  (Variables|Default|SetIsMayPartner false)
  (Variables|Default|SetIsMallowPartner false)
  (Variables|Default|SetIsLilliePartner true)
  (Variables|Default|SetIsLanaPartner false)
  (Variables|Default|SetIsAcerolaPartner false)
  (Class|SkinnedMeshComponent|SetSkeletalMesh _mesh "/Game/MAIN/Pokemon/Trainers/Lily/662.662" true)
  (Class|SkeletalMeshComponent|SetAnimClass _mesh "/Game/MAIN/Pokemon/Trainers/Lily/LillieFollowerAnimBP.LillieFollowerAnimBP_C")
  (Transformation|SetRelativeScale3D _mesh "100.000000,100.000000,100.000000"))

(event Custom|LanaPartnerSelected
  (bind _mesh (Variables|Character|GetMesh))
  (Variables|Default|SetIsRedPartner false)
  (Variables|Default|SetIsSophoclesPartner false)
  (Variables|Default|SetIsMayPartner false)
  (Variables|Default|SetIsMallowPartner false)
  (Variables|Default|SetIsLilliePartner false)
  (Variables|Default|SetIsLanaPartner true)
  (Variables|Default|SetIsAcerolaPartner false)
  (Class|SkinnedMeshComponent|SetSkeletalMesh _mesh "/Game/MAIN/Pokemon/Trainers/Lana/Lana.Lana" true)
  (Class|SkeletalMeshComponent|SetAnimClass _mesh "/Game/MAIN/Pokemon/Trainers/Lana/LanaFollowerAnimBP.LanaFollowerAnimBP_C")
  (Transformation|SetRelativeScale3D _mesh "1.000000,1.000000,1.000000"))

(event Custom|AcerolaPartnerSelected
  (bind _mesh (Variables|Character|GetMesh))
  (Variables|Default|SetIsRedPartner false)
  (Variables|Default|SetIsSophoclesPartner false)
  (Variables|Default|SetIsMayPartner false)
  (Variables|Default|SetIsMallowPartner false)
  (Variables|Default|SetIsLilliePartner false)
  (Variables|Default|SetIsLanaPartner false)
  (Variables|Default|SetIsAcerolaPartner true)
  (Class|SkinnedMeshComponent|SetSkeletalMesh _mesh "/Game/MAIN/Pokemon/Trainers/Purple/666.666" true)
  (Class|SkeletalMeshComponent|SetAnimClass _mesh "/Game/MAIN/Pokemon/Trainers/Purple/PurpleFollowerAnimBP.PurpleFollowerAnimBP_C")
  (Transformation|SetRelativeScale3D _mesh "100.000000,100.000000,100.000000"))

(event EventBeginPlay
  (bind _outactors (Actor|GetAllActorsOfClass "/Game/MAIN/Blueprints/Player/MasterCharacter_BP.MasterCharacter_BP_C"))
  (Variables|Default|SetPlayerReference (Utilities|Array|Get(acopy) _outactors))
  (Utilities|FlowControl|Delay 1.5)
  (CallFunction|CalculatePartnerSkin))

(event Collision|EventActorBeginOverlap
  (params (OtherActor :type Actor%20Object%20Reference)))

(event EventTick
  (params (DeltaSeconds :type Float%20%28single-precision%29))
  (Utilities|FlowControl|Sequence
    (:then_0
      (bind _playerreference (Variables|Default|GetPlayerReference)
        (:then
          (AI|AIMoveTo self "0, 0, 0" _playerreference 2e+02 false))
        (:else)))
    (:then_1
      (bind _playerreference_2 (Variables|Default|GetPlayerReference)
        (:then
          (if (> (Transformation|GetDistanceTo self _playerreference_2) 8e+03)
            (Transformation|SetActorLocation self (Transformation|GetWorldLocation (Variables|/Game/MAIN/Blueprints/Player/MasterCharacter_BP.MasterCharacter_BP_C|GetPetSpawnPoint _playerreference_2)) false false)))
        (:else)))))

(fn ConstructionScript)

(fn CalculatePartnerSkin
  (if (Variables|Default|GetIsRedPartner)
    (CallFunction|RedPartnerSelected)
    (return)
    (elif (Variables|Default|GetIsSophoclesPartner)
      (CallFunction|SophoclesPartnerSelected)
      (return)
      (elif (Variables|Default|GetIsMayPartner)
        (CallFunction|MayPartnerSelected)
        (return)
        (elif (Variables|Default|GetIsMallowPartner)
          (CallFunction|MallowPartnerSelected)
          (return)
          (elif (Variables|Default|GetIsLilliePartner)
            (CallFunction|LilliePartnerSelected)
            (return)
            (elif (Variables|Default|GetIsLanaPartner)
              (CallFunction|LanaPartnerSelected)
              (return)
              (elif (Variables|Default|GetIsAcerolaPartner)
                (CallFunction|AcerolaPartnerSelected)
                (return)
                (else
                  (CallFunction|RedPartnerSelected)
                  (return))))))))))