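; Parent Blueprint for summoned pets that follow the player around, with particle effects on spawn and despawn.
; BeginPlay attaches a temporary spawn emitter to the mesh, while Tick uses DoOnce to start FollowPlayer.
; FollowPlayer runs AIMoveTo toward the player's character or mount, calling itself again on success or failure.
; DespawnMontage optionally plays a slowed montage and briefly reuses the spawn particle, without destroying the pet.
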(event Custom|FollowPlayer
  (bind _returnvalue (Game|GetPlayerCharacter 0))
  (bind _asmaster_character_bp (Utilities|Casting|CastToMasterCharacter_BP _returnvalue)
    (:then
      (AI|AIMoveTo self "0, 0, 0" _asmaster_character_bp 1e+02 false
        (:OnSuccess
          _)
        (:OnFail
          _))
      (CallFunction|FollowPlayer))
    (:CastFailed
      (bind _asmount_parent_bp (Utilities|Casting|CastToMount_Parent_BP _returnvalue))
      (AI|AIMoveTo self "0, 0, 0" _asmount_parent_bp 1e+02 false
        (:OnSuccess
          _)
        (:OnFail
          _))
      (CallFunction|FollowPlayer))))

(event Custom|DespawnMontage
  (if (Variables|Default|GetCanUseDespawnMontage?)
    (Animation|Montage|MontagePlay (Components|SkeletalMesh|GetAnimInstance (Variables|Character|GetMesh)) (Variables|Default|GetDespawnMontageToPlay) 0.1 "MontageLength" 0.0 true)
    (Variables|Default|GetDespawnEmitter
      (:then)
      (:else
        (bind _returnvalue (Effects|SpawnEmitterAttached (Variables|Default|GetSpawnParticle) (Variables|Character|GetMesh) "None" "0, 0, 0" "0, 0, 0" "5.000000,5.000000,5.000000" "SnapToTargetIncludingScale"))
        (Variables|Default|SetDespawnEmitter _returnvalue)
        (Utilities|FlowControl|Delay 0.5)
        (bind _despawnemitter (Variables|Default|GetDespawnEmitter)
          (:then
            (Components|DestroyComponent _despawnemitter))
          (:else))))))

(event EventBeginPlay
  (Variables|Default|GetSpawnEmitter
    (:then)
    (:else
      (bind _returnvalue (Effects|SpawnEmitterAttached (Variables|Default|GetSpawnParticle) (Variables|Character|GetMesh) "None" "0, 0, 0" "0, 0, 0" "5.000000,5.000000,5.000000" "SnapToTargetIncludingScale"))
      (Variables|Default|SetSpawnEmitter _returnvalue)
      (Utilities|FlowControl|Delay 3.8)
      (bind _spawnemitter (Variables|Default|GetSpawnEmitter)
        (:then
          (Components|DestroyComponent _spawnemitter))
        (:else)))))

(event Collision|EventActorBeginOverlap
  (params (OtherActor :type Actor%20Object%20Reference)))

(event EventTick
  (params (DeltaSeconds :type Float%20%28single-precision%29))
  (Utilities|FlowControl|DoOnce false
    (:Completed
      (CallFunction|FollowPlayer))))

(fn ConstructionScript)