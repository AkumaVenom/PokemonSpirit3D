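; Spline movement Blueprint that moves a referenced Actor along a spline in a continuous loop from BeginPlay.
; A timeline, with play rate set by the inverse of TimelineLength, drives distance from the first to last spline point and restarts when finished.
; Each update sets the Actor's world location and orients it along the spline tangent.
; The construction script snaps the Actor to the first spline point.
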(event Custom|PlayTimeline
  (bind _spline (Variables|Default|GetSpline))
  (bind _spline_2 (Variables|Default|GetSpline))
  (bind _actor (Variables|Default|GetActor))
  (Components|Timeline|SetPlayRate (Variables|Default|GetTimeline_0) (/ 1.0 (Variables|Default|GetTimelineLength)))
  (bind _newtrack_2 (Timeline|Timeline_0 PlayFromStart)
    (:Update
      (Transformation|SetActorLocation _actor (Spline|GetLocationatDistanceAlongSpline _spline (Math|Float|Lerp 0.0 (Spline|GetDistanceAlongSplineatSplinePoint _spline_2 (- (Spline|GetNumberOfSplinePoints _spline_2) 1)) _newtrack_2) "World") false false)
      (Transformation|SetActorRotation _actor (Math|Conversions|RotationFromXVector (Spline|GetTangentatDistanceAlongSpline _spline (Math|Float|Lerp 0.0 (Spline|GetDistanceAlongSplineatSplinePoint _spline_2 (- (Spline|GetNumberOfSplinePoints _spline_2) 1)) _newtrack_2) "World"))))
    (:Finished
      (CallFunction|PlayTimeline))))

(event EventBeginPlay
  (CallFunction|PlayTimeline))

(fn ConstructionScript
  (Transformation|SetActorLocation (Variables|Default|GetActor) (Spline|GetLocationatSplinePoint (Variables|Default|GetSpline) 0 "World") false false))